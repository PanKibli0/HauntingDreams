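; Player vitals component that tracks health and sanity.
; Increase and decrease functions clamp each value between zero and its maximum, then broadcast a change event.
; DecreaseHealth also fires a death event at zero health, while sanity has no depletion event.
; The logic setting both values to their maximums is disconnected from BeginPlay, so it never runs.
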(event EventBeginPlay
  ;[1 0.07468 0 0.5] Begin Vitals
)

(fn IncreaseHealth
  (params (Amount :type Float%20%28double-precision%29))
  (bind _output_get (Variables|Default|SetCurrentHealth (Math|Float|Clamp(Float) (+ (Variables|Default|GetCurrentHealth) Amount) 0.0 (Variables|Default|GetMaxHealth))))
  (Default|CallOnHealthChanged _output_get))

(fn DecreaseHealth
  (params (Amount :type Float%20%28double-precision%29))
  (bind _output_get (Variables|Default|SetCurrentHealth (Math|Float|Clamp(Float) (- (Variables|Default|GetCurrentHealth) Amount) 0.0 (Variables|Default|GetMaxHealth))))
  (Default|CallOnHealthChanged _output_get)
  (if (<= (Variables|Default|GetCurrentHealth) 0.0)
    (Default|CallOnDeath)))

(fn IncreaseSanity
  (params (Amount :type Float%20%28double-precision%29))
  (bind _output_get (Variables|Default|SetCurrentSanity (Math|Float|Clamp(Float) (+ (Variables|Default|GetCurrentSanity) Amount) 0.0 (Variables|Default|GetMaxSanity))))
  (Default|CallOnSanityChanged _output_get))

(fn DecreaseSanity
  (params (Amount :type Float%20%28double-precision%29))
  (bind _output_get (Variables|Default|SetCurrentSanity (Math|Float|Clamp(Float) (- (Variables|Default|GetCurrentSanity) Amount) 0.0 (Variables|Default|GetMaxSanity))))
  (Default|CallOnSanityChanged _output_get))