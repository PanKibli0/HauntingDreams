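; Game mode that spawns successive map loops and manages a shared pool of prop actors.
; SpawnNextLoop increments the loop index, spawns a BP_BaseMap at the given attach transform and keeps it as the current loop.
; GetPropFromPool reuses a non-visible pooled actor of the requested class, or spawns and registers a new one.
; ReturnPropToPool detaches props, hides them and disables collision instead of destroying them.
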(fn ConstructionScript)

(fn SpawnNextLoop
  (params (AttachTransform :type Transform))
  (Variables|Default|SetCurrentLoopIndex (+ 1 (Variables|Default|GetCurrentLoopIndex)))
  (bind _returnvalue (Game|SpawnActorfromClass "/Game/Models/Rooms/BP_BaseMap.BP_BaseMap_C" AttachTransform "Undefined" "MultiplyWithRoot" 0 0))
  (bind _output_get (Variables|Default|SetCurrentLoopRef _returnvalue))
  (return _output_get))

(fn GetPropfromPool
  (params (PropClass :type Actor%20Class%20Reference) (PropTransform :type Transform))
  (for _array_element (Variables|Default|GetPropPool)
    (Utilities|IsValid _array_element
      (:Is%20Valid
        (if (and (not (Rendering|IsVisible (Variables|/Script/Engine.Actor|GetRootComponent _array_element))) (== (Utilities|GetClass _array_element) PropClass))
          (Transformation|SetActorTransform _array_element PropTransform)
          (Rendering|SetActorHiddenInGame _array_element false)
          (Collision|SetActorEnableCollision _array_element true)
          (return _array_element)))))
  (bind _returnvalue (Game|SpawnActorfromClass PropClass PropTransform "Undefined" "MultiplyWithRoot" 0 0))
  (Utilities|Array|Add (Variables|Default|GetPropPool) _returnvalue)
  (return _returnvalue))

(fn ReturnProptoPool
  (params (TargetActor :type Actor%20Object%20Reference))
  (Transformation|DetachFromActor TargetActor "KeepWorld" "KeepWorld" "KeepWorld")
  (Rendering|SetActorHiddenInGame TargetActor true)
  (Collision|SetActorEnableCollision TargetActor false))