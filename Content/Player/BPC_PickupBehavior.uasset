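; Actor component that lets its owning actor be picked up and dropped in the world.
; On pickup it caches the static mesh's collision mode, then hides the mesh with its children and disables collision.
; On drop it moves the owner to the given location without sweeping, shows the mesh again and restores the cached collision mode.
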(fn OnPickedUp
  (bind _returnvalue (Components|GetOwner))
  (bind _returnvalue_2 (Actor|GetComponentbyClass _returnvalue "/Script/Engine.StaticMeshComponent"))
  (Variables|Default|SetCachedCollisionType%20 (Collision|GetCollisionEnabled _returnvalue_2))
  (Rendering|SetVisibility _returnvalue_2 false true)
  (Collision|SetCollisionEnabled _returnvalue_2 "NoCollision"))

(fn OnDropped
  (params (Location :type Vector))
  (bind _returnvalue (Components|GetOwner))
  (bind _returnvalue_2 (Actor|GetComponentbyClass _returnvalue "/Script/Engine.StaticMeshComponent"))
  (Transformation|SetActorLocation _returnvalue Location false false)
  (Rendering|SetVisibility _returnvalue_2 true true)
  (Collision|SetCollisionEnabled _returnvalue_2 (Variables|Default|GetCachedCollisionType%20)))