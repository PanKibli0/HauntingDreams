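; First-person player character with walking, sprint, crouch, climbing, mantling, door and interface interactions, physics-handle grabbing and a flashlight.
; Upward input line-traces from the camera to climb BP_Climbable surfaces, mantle validated ledges, or call HandleJump, whose logic is disconnected.
; Climbing uses Flying mode, wall traces and limited camera yaw.
; Tick drives wall-to-mantle transitions, interpolated mantle movement with capsule collision set to query-only, and held-object positioning.
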(event Custom|StopClimbing
  ;[1 0 0.489 0.5] Stop Climbing
  (if (Variables|State|GetIsClimbing)
    (Variables|State|SetIsClimbing false)
    (Pawn|Components|CharacterMovement|SetMovementMode (Variables|Character|GetCharacterMovement) "MOVE_Falling" 0)
    (Transformation|SetActorRotation (Math|Rotator|MakeRotator 0.0 0.0 (.yaw (Transformation|GetActorRotation))))
    (CallFunction|CameraLimitReset)
    (Variables|Climbing|SetWallHitLocation "0, 0, 0")
    (Variables|Climbing|SetClimbWallNormal "0, 0, 0")))

(event Custom|ClimbLoop
  ;[0.15 0.15 0.15 0.5] Climb loop
  (if (Variables|State|GetIsClimbing) ; Hit
    (bind (_out_hit _is_hit) (CallFunction|LineTrace (Variables|Collision|GetCapsuleComponent) 1.2e+02))
    (if _is_hit
      (Variables|Climbing|SetLastVerticalWallHitLocation (.Location (Collision|BreakHitResult _out_hit)))
      (Variables|Climbing|SetLastVerticalWallNormal (.Normal (Collision|BreakHitResult _out_hit)))
      (Utilities|Casting|CastToBP_Climbable (.HitActor (Collision|BreakHitResult _out_hit))
        (:then
          (Transformation|SetActorRotation (|RInterp)))
        (:CastFailed
          (bind (_canmantle _targetlocation_) (CallFunction|CheckCanMantle (Variables|Climbing|GetLastVerticalWallHitLocation) (Variables|Climbing|GetLastVerticalWallNormal)))
          (if _canmantle
            (CallFunction|HandleMantle _targetlocation_)))))))

(event Custom|MantleLoop
  (bind _returnvalue (Transformation|GetActorLocation))
  ;[1 0.9224 0.2834 0.5] Mantle Loop
  (if (Variables|State|GetIsMantling)
    (if (Utilities|Operators|EqualEqual (Transformation|GetActorLocation) (Math|Vector|MakeVector (.x _returnvalue) (.y _returnvalue) (.z (Variables|Helpers|GetMantleTargetLocation))) 1.0)
      (Transformation|SetActorLocation (Math|Interpolation|VInterpTo (Transformation|GetActorLocation) (Variables|Helpers|GetMantleTargetLocation) (Variables|Helpers|GetdeltaTIme) 12.0) false false) ; Up
      (if (Utilities|Operators|EqualEqual (Transformation|GetActorLocation) (Variables|Helpers|GetMantleTargetLocation) 0.1)
        (Pawn|Components|CharacterMovement|SetMovementMode (Variables|Character|GetCharacterMovement) "MOVE_Falling" 0)
        (Variables|State|SetIsMantling false)
        (Collision|SetCollisionEnabled (Variables|Collision|GetCapsuleComponent) "QueryAndPhysics"))
      (else
        (Transformation|SetActorLocation (Math|Interpolation|VInterpTo (Transformation|GetActorLocation) (Variables|Helpers|GetMantleTargetLocation) (Variables|Helpers|GetdeltaTIme) 12.0) false false) ; forward
      ))))

(event Custom|Holding
  (bind _camera (Variables|Default|GetCamera))
  ;[0.15 0.15 0.15 0.5] Holding
  (if (Variables|State|GetIs%20Holding)
    (Physics|Components|PhysicsHandle|SetTargetLocation (Variables|Default|GetPhysicsHandle) (+ (Transformation|GetWorldLocation _camera) (* (Math|Vector|GetForwardVector (Transformation|GetWorldRotation _camera)) 2.5e+02)))))

(event Input|EnhancedActionEvents|EnhancedInputActionIA_UpwardAction
  (params (ActionValue :type Boolean) (ElapsedSeconds :type Float%20%28double-precision%29) (TriggeredSeconds :type Float%20%28double-precision%29) (InputAction :type Input%20Action%20Object%20Reference :default "/Game/Input/Actions/IA_UpwardAction.IA_UpwardAction"))
  ;[0.15 0.15 0.15 0.5] IA_UpWard - Jump, Climb, Vault
  (:Started
    (bind (_out_hit _is_hit) (CallFunction|LineTrace (Variables|Default|GetCamera) 1e+02))
    (if _is_hit ; Hit
      (Utilities|Casting|CastToBP_Climbable (.HitActor (Collision|BreakHitResult _out_hit))
        (:then
          (if (not (Variables|State|GetIsClimbing))
            (CallFunction|HandleClimb (.Location (Collision|BreakHitResult _out_hit)) (.Normal (Collision|BreakHitResult _out_hit)))))
        (:CastFailed
          (bind (_canmantle _targetlocation_) (CallFunction|CheckCanMantle (.Location (Collision|BreakHitResult _out_hit)) (.Normal (Collision|BreakHitResult _out_hit))))
          (if _canmantle
            (CallFunction|HandleMantle _targetlocation_)
            (else
              (CallFunction|HandleJump :!label _label)))))
      (else
        (goto _label))))
  (:Completed
    (Character|StopJumping)))

(event Input|EnhancedActionEvents|EnhancedInputActionIA_CameraLook
  (params (ActionValue :type Vector%202D%20Structure) (ElapsedSeconds :type Float%20%28double-precision%29) (TriggeredSeconds :type Float%20%28double-precision%29) (InputAction :type Input%20Action%20Object%20Reference :default "/Game/Input/Actions/IA_CameraLook.IA_CameraLook"))
  ;[1 0.00718 0.7418] Camera
  (Pawn|Input|AddControllerYawInput (.x ActionValue)) ; LEFT/RIGHT
  (Pawn|Input|AddControllerPitchInput (* (.y ActionValue) -1.0)) ; UP/DOWN
)

(event Input|EnhancedActionEvents|EnhancedInputActionIA_Move
  (params (ActionValue :type Vector%202D%20Structure) (ElapsedSeconds :type Float%20%28double-precision%29) (TriggeredSeconds :type Float%20%28double-precision%29) (InputAction :type Input%20Action%20Object%20Reference :default "/Game/Input/Actions/IA_Move.IA_Move"))
  ;[1 1 1 0.5] Movement
  ;;[0 0.2067 0.1591] Basic Movement
  ;;[0 0.2067 0.1591] ClimbMovement
  (if (not (Variables|State|GetIsMantling))
    (if (Variables|State|GetIsClimbing)
      (CallFunction|ClimbMovement (.x ActionValue) (.y ActionValue))
      (else
        (Pawn|Input|AddMovementInput (Transformation|GetActorRightVector) (.x ActionValue) false) ; LEFT/RIGHT
        (Pawn|Input|AddMovementInput (Transformation|GetActorForwardVector) (.y ActionValue) false) ; FORWARD/BACKWARD
      ))))

(event Input|EnhancedActionEvents|EnhancedInputActionIA_Interaction
  (params (ActionValue :type Boolean) (ElapsedSeconds :type Float%20%28double-precision%29) (TriggeredSeconds :type Float%20%28double-precision%29) (InputAction :type Input%20Action%20Object%20Reference :default "/Game/Input/Actions/IA_Interaction.IA_Interaction"))
  ;[0.15 0.15 0.15 0.5] Interact
  (:Started
    (bind (_out_hit _is_hit) (CallFunction|LineTrace (Variables|Default|GetCamera) 2e+02))
    (Utilities|FlowControl|Sequence
      (:then_0
        (if _is_hit
          (if (Utilities|DoesObjectImplementInterface (.HitActor (Collision|BreakHitResult _out_hit)) "/Game/Player/BPI_Interactions.BPI_Interactions_C")
            (Class|BPIInteractions|Interact(Message) (.HitActor (Collision|BreakHitResult _out_hit))))))
      (:then_1
        (Utilities|IsValid (.HitActor (Collision|BreakHitResult _out_hit))
          (:Is%20Valid
            (if (Actor|ActorHasTag (.HitActor (Collision|BreakHitResult _out_hit)) "Door")
              (bind _asbp_door (Utilities|Casting|CastToBP_Door (.HitActor (Collision|BreakHitResult _out_hit))))
              (Default|OpenDoor _asbp_door))))))))

(event Input|EnhancedActionEvents|EnhancedInputActionIA_StopClimb
  (params (ActionValue :type Boolean) (ElapsedSeconds :type Float%20%28double-precision%29) (TriggeredSeconds :type Float%20%28double-precision%29) (InputAction :type Input%20Action%20Object%20Reference :default "/Game/Input/Actions/IA_StopClimb.IA_StopClimb"))
  ;[1 0 0.489 0.5] Stop Climbing
  (if (Variables|State|GetIsClimbing)
    (Variables|State|SetIsClimbing false)
    (Pawn|Components|CharacterMovement|SetMovementMode (Variables|Character|GetCharacterMovement) "MOVE_Falling" 0)
    (Transformation|SetActorRotation (Math|Rotator|MakeRotator 0.0 0.0 (.yaw (Transformation|GetActorRotation))))
    (CallFunction|CameraLimitReset)
    (Variables|Climbing|SetWallHitLocation "0, 0, 0")
    (Variables|Climbing|SetClimbWallNormal "0, 0, 0")))

(event Input|EnhancedActionEvents|EnhancedInputActionIA_Crouch
  (params (ActionValue :type Boolean) (ElapsedSeconds :type Float%20%28double-precision%29) (TriggeredSeconds :type Float%20%28double-precision%29) (InputAction :type Input%20Action%20Object%20Reference :default "/Game/Input/Actions/IA_Crouch.IA_Crouch"))
  ;[0.15 0 0.01997 0.5] Crouch
  (:Started
    (if (not (or (AI|Components|NavMovement|IsFalling (Variables|Character|GetCharacterMovement)) (Variables|State|GetIsClimbing)))
      (Utilities|FlowControl|FlipFlop
        (:A
          (Character|Crouch)
          (Variables|State|SetIsCrounching true))
        (:B
          (Character|UnCrouch)
          (Variables|State|SetIsCrounching false))))))

(event Input|EnhancedActionEvents|EnhancedInputActionIA_Sprint
  (params (ActionValue :type Boolean) (ElapsedSeconds :type Float%20%28double-precision%29) (TriggeredSeconds :type Float%20%28double-precision%29) (InputAction :type Input%20Action%20Object%20Reference :default "/Game/Input/Actions/IA_Sprint.IA_Sprint"))
  (bind _charactermovement (Variables|Character|GetCharacterMovement))
  ;[0.15 0 0.01997 0.5] Sprint
  (:Started
    (Variables|/Script/Engine.CharacterMovementComponent|SetMaxWalkSpeed _charactermovement (Variables|Speed|GetMaxSprintSpeed)))
  (:Completed
    (Variables|/Script/Engine.CharacterMovementComponent|SetMaxWalkSpeed _charactermovement (Variables|Speed|GetMaxSpeed))))

(event Input|EnhancedActionEvents|EnhancedInputActionIA_FlashLight
  (params (ActionValue :type Boolean) (ElapsedSeconds :type Float%20%28double-precision%29) (TriggeredSeconds :type Float%20%28double-precision%29) (InputAction :type Input%20Action%20Object%20Reference :default "/Game/Input/Actions/IA_FlashLight.IA_FlashLight"))
  ;[1 0.8744 0 0.5] FlashLight
  (Rendering|ToggleVisibility (Variables|Default|GetFlashlight) false))

(event EventTick
  (params (DeltaSeconds :type Float%20%28single-precision%29))
  ;[0.15 0 0.06308 0.5] Event Tick
  (Variables|Helpers|SetdeltaTIme DeltaSeconds)
  (Utilities|FlowControl|Sequence
    (:then_0
      (CallFunction|ClimbLoop))
    (:then_1
      (CallFunction|MantleLoop))
    (:then_2
      (CallFunction|Holding))))

(event EventBeginPlay
  ;[0.15 0 0.01997 0.5] Input Controls
  (bind _asplayer_controller (Utilities|Casting|CastToPlayerController (Pawn|GetController)))
  (Utilities|IsValid (PlayerController|LocalPlayerSubsystems|GetEnhancedInputLocalPlayerSubsystem _asplayer_controller)
    (:Is%20Valid
      (Input|AddMappingContext (PlayerController|LocalPlayerSubsystems|GetEnhancedInputLocalPlayerSubsystem _asplayer_controller) "/Game/Input/IMC_Default.IMC_Default" 0 "(bIgnoreAllPressedKeysUntilRelease=True,bForceImmediately=False,bNotifyUserSettings=False)"))))

(event Input|KeyboardEvents|F
  (params (Key :type Key%20Structure :default "None"))
  (bind _camera (Variables|Default|GetCamera))
  (bind _returnvalue (Transformation|GetWorldLocation _camera))
  ;[0.15 0.15 0.15 0.5] Grabbing
  (:Pressed
    (bind (_outhit _returnvalue_2) (Collision|LineTraceByChannel _returnvalue (+ _returnvalue (* (Math|Vector|GetForwardVector _camera) 3e+02)) "TraceTypeQuery1" false 0 "None"))
    (if _returnvalue_2
      (Physics|Components|PhysicsHandle|GrabComponentatLocationwithRotation (Variables|Default|GetPhysicsHandle) (.HitComponent (Collision|BreakHitResult _outhit)) "None" (Transformation|GetWorldLocation (.HitComponent (Collision|BreakHitResult _outhit))) "0, 0, 0")
      (Variables|State|SetIs%20Holding true)))
  (:Released
    (if (Variables|State|GetIs%20Holding)
      (Physics|Components|PhysicsHandle|ReleaseComponent (Variables|Default|GetPhysicsHandle))
      (Variables|State|SetIs%20Holding (Variables|State|GetIs%20Holding)))))

(fn ConstructionScript)

(fn SphereTrace
  (params (Start%20Component :type Scene%20Component%20Object%20Reference) (Distance :type Float%20%28double-precision%29) (Radius :type Float%20%28double-precision%29))
  (bind _returnvalue (Transformation|GetWorldLocation Start%20Component))
  (bind (_outhit _returnvalue_2) (Collision|SphereTraceByChannel _returnvalue (+ _returnvalue (* (Math|Vector|GetForwardVector (Transformation|GetWorldRotation Start%20Component)) Distance)) Radius "TraceTypeQuery1" false 0 "None"))
  (return _outhit _returnvalue_2))

(fn HandleJump)

(fn LineTrace
  (params (StartComponent :type Scene%20Component%20Object%20Reference) (Distance :type Float%20%28double-precision%29))
  (bind _returnvalue (Transformation|GetWorldLocation StartComponent))
  (bind (_outhit _returnvalue_2) (Collision|LineTraceByChannel _returnvalue (+ _returnvalue (* (Math|Vector|GetForwardVector (Transformation|GetWorldRotation StartComponent)) Distance)) "TraceTypeQuery1" false 0 "ForDuration"))
  (return _outhit _returnvalue_2))

(fn HandleClimb
  (params (HitLocation :type Vector) (HitNormal :type Vector))
  (if (Variables|State|GetIsCrounching)
    (Variables|State|SetIsCrounching false)
    (Character|UnCrouch))
  (Variables|State|SetIsClimbing true)
  (Variables|Climbing|SetWallHitLocation HitLocation)
  (Variables|Climbing|SetClimbWallNormal HitNormal)
  (CallFunction|ClimbCameraLimit)
  (Pawn|Components|CharacterMovement|SetMovementMode (Variables|Character|GetCharacterMovement) "MOVE_Flying" 0)
  (Transformation|SetActorLocationAndRotation (+ HitLocation (* HitNormal (Variables|Climbing|GetClimbingDistancePosition))) (Math|Rotator|MakeRotator 0.0 0.0 (.yaw (Math|Rotator|MakeRotfromX (* HitNormal -1.0))))))

(fn ClimbCameraLimit
  (bind _climbwallnormal (Variables|Climbing|GetClimbWallNormal))
  (bind _returnvalue (* _climbwallnormal -1.0))
  (bind _returnvalue_2 (Math|Rotator|MakeRotfromX _returnvalue))
  (bind _asplayer_controller (Utilities|Casting|CastToPlayerController (Pawn|GetController)))
  (Variables|Default|SetbUseControllerRotationYaw false)
  (Variables|/Script/Engine.PlayerCameraManager|SetViewYawMin (Variables|/Script/Engine.PlayerController|GetPlayerCameraManager _asplayer_controller) (- (.yaw _returnvalue_2) 1.2e+02))
  (Variables|/Script/Engine.PlayerCameraManager|SetViewYawMax (Variables|/Script/Engine.PlayerController|GetPlayerCameraManager _asplayer_controller) (+ (.yaw _returnvalue_2) 1.2e+02)))

(fn CameraLimitReset
  (bind _asplayer_controller (Utilities|Casting|CastToPlayerController (Pawn|GetController)))
  (Variables|Default|SetbUseControllerRotationYaw true)
  (Variables|/Script/Engine.PlayerCameraManager|SetViewYawMin (Variables|/Script/Engine.PlayerController|GetPlayerCameraManager _asplayer_controller) 0.0)
  (Variables|/Script/Engine.PlayerCameraManager|SetViewYawMax (Variables|/Script/Engine.PlayerController|GetPlayerCameraManager _asplayer_controller) 359.99))

(fn CheckHorizontalClimb
  (params (Input%20X :type Float%20%28double-precision%29))
  (bind _returnvalue (Transformation|GetActorLocation))
  (bind (_outhit _returnvalue_2) (Collision|LineTraceByChannel _returnvalue (+ (* (Math|Vector|GetForwardVector (Math|Rotator|CombineRotators (Transformation|GetActorRotation) (Math|Rotator|MakeRotator 0.0 0.0 (* Input%20X 4e+01)))) 1.5e+02) _returnvalue) "TraceTypeQuery1" false 0 "ForDuration" true "(R=0.010613,G=0.005887,B=1.000000,A=1.000000)"))
  (if _returnvalue_2
    (Utilities|Casting|CastToBP_Climbable (.HitActor (Collision|BreakHitResult _outhit))
      (:then
        (if (Utilities|Operators|EqualEqual (Variables|Climbing|GetClimbWallNormal) (.Normal (Collision|BreakHitResult _outhit)) 0.05)
          _
          (else
            (Variables|Climbing|SetClimbWallNormal (.Normal (Collision|BreakHitResult _outhit)))
            (Variables|Climbing|SetWallHitLocation (.ImpactPoint (Collision|BreakHitResult _outhit)))
            (CallFunction|ClimbCameraLimit)))
        (return true))
      (:CastFailed
        _)))
  (return false))

(fn CheckShouldStopClimb
  (bind _returnvalue (Transformation|GetActorLocation))
  (bind _returnvalue_2 (Collision|LineTraceByChannel _returnvalue (- _returnvalue (* "0.000000,0.000000,1.000000" (+ (Components|Capsule|GetScaledCapsuleHalfHeight (Variables|Collision|GetCapsuleComponent)) 25.0))) "TraceTypeQuery1" false 0 "ForDuration" true "(R=1.000000,G=0.879337,B=0.028836,A=1.000000)" "(R=0.000000,G=1.000000,B=0.000000,A=1.000000)" 1e+02))
  (if _returnvalue_2
    (Development|PrintString (Utilities|String|Append "Stop CLimbing: " (Utilities|String|ToString(Boolean) _returnvalue_2)) true true "(R=1.000000,G=0.000000,B=0.024331,A=1.000000)" 0.5)
    (else
      (Development|PrintString (Utilities|String|Append "Stop CLimbing: " (Utilities|String|ToString(Boolean) _returnvalue_2)) true true "(R=0.000000,G=0.660000,B=1.000000,A=1.000000)" 0.5)))
  (return _returnvalue_2))

(fn ClimbMovement
  (params (Input%20X :type Float%20%28double-precision%29) (Input%20Y :type Float%20%28double-precision%29))
  (if (!= Input%20X 0.0)
    (bind _can_move (CallFunction|CheckHorizontalClimb Input%20X))
    (bind _output_get (Variables|Climbing|SetHorizontalClimb _can_move))
    (if _output_get
      (Pawn|Input|AddMovementInput (Transformation|GetActorRightVector) Input%20X false :!label _label) ; LEFT/RIGHT CLIMB
    )
    (else
      (goto _label)))
  (if (< Input%20Y 0.0)
    (bind _stopclimbing (CallFunction|CheckShouldStopClimb))
    (if _stopclimbing
      (CallFunction|StopClimbing)
      (else
        (Pawn|Input|AddMovementInput (Transformation|GetActorUpVector) Input%20Y false :!label _label_2) ; UP/DOWN CLIMB
        (|Position)))
    (else
      (goto _label_2))))

(fn CheckCanMantle
  (params (WallHitLocation :type Vector) (WallNormal :type Vector))
  (bind _returnvalue (* WallNormal -4e+01))
  (bind _returnvalue_2 (+ WallHitLocation "0.000000,0.000000,80.000000"))
  (bind _capsulecomponent (Variables|Collision|GetCapsuleComponent))
  (bind _returnvalue_3 (Components|Capsule|GetScaledCapsuleHalfHeight _capsulecomponent))
  (bind _returnvalue_4 (+ _returnvalue_2 _returnvalue))
  (bind _outhit (Collision|LineTraceByChannel _returnvalue_4 (- _returnvalue_4 "0.000000,0.000000,200.000000") "TraceTypeQuery1" false 0 "ForDuration" true "(R=0.272549,G=0.000000,B=0.520028,A=1.000000)" "(R=0.000000,G=1.000000,B=0.000000,A=1.000000)" 1e+03))
  (if (.bBlockingHit (Collision|BreakHitResult _outhit))
    (if (Math|Float|InRange(Float) (- (.Z (Math|Vector|BreakVector (.Location (Collision|BreakHitResult _outhit)))) (.z (Transformation|GetActorLocation))) 5e+01 2e+02)
      (bind _returnvalue_5 (Collision|CapsuleTraceByChannel (Math|Vector|MakeVector (.X (Math|Vector|BreakVector (+ (.Location (Collision|BreakHitResult _outhit)) (* WallNormal -2e+01)))) (.Y (Math|Vector|BreakVector (+ (.Location (Collision|BreakHitResult _outhit)) (* WallNormal -2e+01)))) (+ (.Z (Math|Vector|BreakVector (+ (.Location (Collision|BreakHitResult _outhit)) (* WallNormal -2e+01)))) _returnvalue_3 15.0)) (Math|Vector|MakeVector (.X (Math|Vector|BreakVector (+ (.Location (Collision|BreakHitResult _outhit)) (* WallNormal -2e+01)))) (.Y (Math|Vector|BreakVector (+ (.Location (Collision|BreakHitResult _outhit)) (* WallNormal -2e+01)))) (+ (.Z (Math|Vector|BreakVector (+ (.Location (Collision|BreakHitResult _outhit)) (* WallNormal -2e+01)))) _returnvalue_3 15.0)) (Components|Capsule|GetScaledCapsuleRadius _capsulecomponent) _returnvalue_3 "TraceTypeQuery1" false 0 "Persistent" true "(R=0.904505,G=1.000000,B=0.959935,A=1.000000)" "(R=0.000000,G=1.000000,B=0.000000,A=1.000000)" 1e+03))
      (if _returnvalue_5
        (return false "0, 0, 0")
        (else
          (Development|PrintString "MANTLE")
          (return true (Math|Vector|MakeVector (.X (Math|Vector|BreakVector (+ (.Location (Collision|BreakHitResult _outhit)) (* WallNormal -2e+01)))) (.Y (Math|Vector|BreakVector (+ (.Location (Collision|BreakHitResult _outhit)) (* WallNormal -2e+01)))) (+ (.Z (Math|Vector|BreakVector (+ (.Location (Collision|BreakHitResult _outhit)) (* WallNormal -2e+01)))) _returnvalue_3 15.0)))))
      (else
        (return false "0, 0, 0")))
    (else
      (return false "0, 0, 0"))))

(fn HandleMantle
  (params (TargetLocation :type Vector))
  (Variables|Helpers|SetMantleTargetLocation TargetLocation)
  (Variables|State|SetIsMantling true)
  (Pawn|Components|CharacterMovement|SetMovementMode (Variables|Character|GetCharacterMovement) "MOVE_Flying" 0)
  (Collision|SetCollisionEnabled (Variables|Collision|GetCapsuleComponent) "QueryOnly"))