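; BP_EventAction_Sound is an event action actor in the events system that plays a configured sound at its own location.
; On execute it casts its ActionConfig to DA_EventActionConfig_Sound, spawns the sound with that asset's volume and attenuation, and prints the sound's name.
; It waits for the sound's duration, then signals the event finished and destroys itself.
; A missing or wrong config finishes and destroys immediately.
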(event EventExecuteEvent
  (bind _asda_event_action_config_sound (Utilities|Casting|CastToDA_EventActionConfig_Sound (Variables|Default|GetActionConfig))
    (:then
      (if (Utilities|IsValid _asda_event_action_config_sound)
        (Audio|SpawnSoundatLocation (Variables|/Game/Blueprints/EventsSystem/DataAssets/DA_EventActionConfig_Sound.DA_EventActionConfig_Sound_C|GetSoundToPlay _asda_event_action_config_sound) (Transformation|GetActorLocation) "0, 0, 0" (Variables|/Game/Blueprints/EventsSystem/DataAssets/DA_EventActionConfig_Sound.DA_EventActionConfig_Sound_C|GetVolume _asda_event_action_config_sound) 1.0 0.0 (Variables|/Game/Blueprints/EventsSystem/DataAssets/DA_EventActionConfig_Sound.DA_EventActionConfig_Sound_C|GetSoundAttenuation _asda_event_action_config_sound) 0)
        (Development|PrintString (Utilities|GetDisplayName (Variables|/Game/Blueprints/EventsSystem/DataAssets/DA_EventActionConfig_Sound.DA_EventActionConfig_Sound_C|GetSoundToPlay _asda_event_action_config_sound)))
        (Utilities|FlowControl|Delay (Variables|/Script/Engine.SoundBase|GetDuration (Variables|/Game/Blueprints/EventsSystem/DataAssets/DA_EventActionConfig_Sound.DA_EventActionConfig_Sound_C|GetSoundToPlay _asda_event_action_config_sound)))
        (Default|CallOnEventFinished)
        (Actor|DestroyActor)
        (else
          (Default|CallOnEventFinished)
          (Actor|DestroyActor))))
    (:CastFailed
      (Default|CallOnEventFinished)
      (Actor|DestroyActor))))

(fn ConstructionScript
  (|CallParentFunction))