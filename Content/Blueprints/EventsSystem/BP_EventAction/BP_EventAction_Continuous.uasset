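; BP_EventAction_Continuous is an event action in the events system for effects that repeat until stopped, currently a stub with an empty tick handler.
; ExecuteEvent casts the action config to DA_EventActionConfig_Base, prints a debug message and starts a looping timer that uses the config's Duration as its interval.
; StopEvent clears that timer, then calls the parent stop logic.
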(event Custom|OnContinuousTick)

(event EventExecuteEvent
  (bind _asda_event_action_config_base (Utilities|Casting|CastToDA_EventActionConfig_Base (Variables|Default|GetActionConfig)))
  (Development|PrintString "Hello")
  (bind _returnvalue (Utilities|Time|SetTimerbyEvent (delegate Custom|OnContinuousTick) (Variables|/Game/Blueprints/EventsSystem/DataAssets/DA_EventActionConfig_Base.DA_EventActionConfig_Base_C|GetDuration _asda_event_action_config_base) true))
  (Variables|Default|SetTimerHandle _returnvalue))

(event EventStopEvent
  (Utilities|Time|ClearandInvalidateTimerbyHandle (Variables|Default|GetTimerHandle))
  (|CallParentFunction))

(fn ConstructionScript
  (|CallParentFunction))