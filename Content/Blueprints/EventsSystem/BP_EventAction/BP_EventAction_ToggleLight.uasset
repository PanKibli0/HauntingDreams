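; Event action that temporarily changes lights on target actors for the event system, using a DA_EventActionConfig_Light config.
; ExecuteEvent collects target and tag-matched actors without duplicates, casts one generic component lookup per actor to LightComponent, then applies intensity and color and toggles visibility.
; After the configured duration it toggles visibility again, signals completion and destroys itself; a wrong config type finishes immediately.
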(event EventExecuteEvent
  (bind _asda_event_action_config_light (Utilities|Casting|CastToDA_EventActionConfig_Light (Variables|Default|GetActionConfig))
    (:then
      (for _array_element (Variables|Default|GetTargetActors)
        (Utilities|Array|AddUnique (Variables|Default|GetCollectedActors) _array_element)
        (if (|LengthTags) ; Use Tags
          (for _array_element_2 (Variables|Default|GetTargetTags%20)
            (bind _outactors (Actor|GetAllActorswithTag _array_element_2))
            (for _array_element_3 _outactors
              (Utilities|Array|AddUnique (Variables|Default|GetCollectedActors) _array_element_3))))
        (for _array_element_4 (Variables|Default|GetCollectedActors) ; Lights
          (if true
            (bind _aslight_component (Utilities|Casting|CastToLightComponent (Actor|GetComponentbyClass _array_element_4 "/Script/Engine.ActorComponent")))
            (Rendering|Components|Light|SetIntensity _aslight_component (Variables|/Game/Blueprints/EventsSystem/DataAssets/DA_EventActionConfig_Light.DA_EventActionConfig_Light_C|GetIntensity _asda_event_action_config_light))
            (Rendering|Components|Light|SetLightColor _aslight_component (Variables|/Game/Blueprints/EventsSystem/DataAssets/DA_EventActionConfig_Light.DA_EventActionConfig_Light_C|GetLightColor _asda_event_action_config_light) true)
            (Rendering|ToggleVisibility _aslight_component false)))
        (Utilities|FlowControl|Delay (Variables|/Game/Blueprints/EventsSystem/DataAssets/DA_EventActionConfig_Base.DA_EventActionConfig_Base_C|GetDuration _asda_event_action_config_light))
        (for _array_element_5 (Variables|Default|GetCollectedActors)
          (if true
            (bind _aslight_component_2 (Utilities|Casting|CastToLightComponent (Actor|GetComponentbyClass _array_element_5 "/Script/Engine.ActorComponent")))
            (Rendering|ToggleVisibility _aslight_component_2 false)))
        (Default|CallOnEventFinished)
        (Actor|DestroyActor)))
    (:CastFailed
      (Default|CallOnEventFinished)
      (Actor|DestroyActor))))

(fn ConstructionScript
  (|CallParentFunction))