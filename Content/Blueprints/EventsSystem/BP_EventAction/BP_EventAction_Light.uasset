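; Event action Blueprint that flickers the lights in its TargetActors for a set time.
; ExecuteEvent starts a self-looping Delay that toggles each Light actor's component visibility every FlickerDuration.
; A parallel Sequence branch waits for Duration, signals that the event finished and destroys the action actor.
; Light visibility is not restored at the end, so lights stay in whatever state the last toggle left.
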(event EventExecuteEvent
  (Utilities|FlowControl|Sequence
    (:then_0
      (for _array_element (Variables|Default|GetTargetActors) :!label _label
        (bind _aslight (Utilities|Casting|CastToLight _array_element))
        (Rendering|ToggleVisibility (Variables|/Script/Engine.Light|GetLightComponent _aslight) false))
      (Utilities|FlowControl|Delay (Variables|Default|GetFlickerDuration))
      (goto _label))
    (:then_1
      (Utilities|FlowControl|Delay (Variables|Default|GetDuration))
      (Default|CallOnEventFinished)
      (Actor|DestroyActor))))

(fn ConstructionScript
  (|CallParentFunction))