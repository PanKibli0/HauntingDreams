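; Base trigger actor for the events system that broadcasts an OnPlayerEntered dispatcher when an actor overlaps it.
; On BeginPlay it finds and caches a reference to the level's BP_EventManager.
; TriggerOnce and HasTriggered optionally limit it to a single firing.
; The overlapping actor is passed along without any check that it is the player.
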(event EventBeginPlay
  (bind _returnvalue (Actor|GetActorOfClass "/Game/Blueprints/EventsSystem/BP_EventManager.BP_EventManager_C"))
  (bind _asbp_event_manager (Utilities|Casting|CastToBP_EventManager _returnvalue))
  (Variables|Default|SetEventManagerRef _asbp_event_manager))

(event Collision|EventActorBeginOverlap
  (params (OtherActor :type Actor%20Object%20Reference))
  (if (not (and (Variables|Default|GetTriggerOnce) (Variables|Default|GetHasTriggered)))
    (Variables|Default|SetHasTriggered true)
    (Variables|Default|SetHasTriggered true)
    (Default|CallOnPlayerEntered OtherActor)))

(fn ConstructionScript)