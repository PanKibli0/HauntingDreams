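; AI controller for the cockroach that runs BT_Cockroach on possess and feeds its blackboard from AI perception.
; Seeing the player sets TargetActor and cancels any pending clear timer, while losing sight of an actor clears the target immediately.
; Sighting a non-player actor starts a short timer that clears the target.
; Successfully heard stimuli write their location to HeardSoundLocation.
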(event OnTargetPerceptionUpdated(AIPerception)
  (params (Actor :type Actor%20Object%20Reference) (Stimulus :type AI%20Stimulus%20Structure))
  (bind (_age _expirationage _strength _stimuluslocation _receiverlocation _tag _bsuccessfullysensed) (Utilities|Struct|BreakAIStimulus Stimulus))
  (bind _blackboard (Variables|Default|GetBlackboard))
  (bind _targetactor (Variables|Default|GetTargetActor))
  (bind _returnvalue (Class|AIPerceptionSystem|GetSenseClassforStimulus Stimulus))
  (if (== _returnvalue "/Script/AIModule.AISense_Sight")
    (if _bsuccessfullysensed
      (bind _asbp_player (Utilities|Casting|CastToBP_Player Actor)
        (:then
          (AI|Components|Blackboard|SetValueasObject _blackboard _targetactor _asbp_player)
          (Utilities|Time|ClearandInvalidateTimerbyHandle (Variables|Default|GetLoseSightTimerHandle)))
        (:CastFailed
          (bind _returnvalue_2 (Utilities|Time|SetTimerbyEvent (delegate Custom|ClearTarget) 3.0))
          (Variables|Default|SetLoseSightTimerHandle _returnvalue_2)))
      (else
        (AI|Components|Blackboard|SetValueasObject _blackboard _targetactor 0)))
    (elif (== _returnvalue "/Script/AIModule.AISense_Hearing")
      (if _bsuccessfullysensed
        (AI|Components|Blackboard|SetValueasVector (Variables|Default|GetBlackboard) (Variables|Default|GetHeardSoundLocation) _stimuluslocation)))))

(event Custom|ClearTarget
  (Utilities|Time|ClearandInvalidateTimerbyHandle (Variables|Default|GetLoseSightTimerHandle))
  (AI|Components|Blackboard|SetValueasObject (Variables|Default|GetBlackboard) (Variables|Default|GetTargetActor) 0))

(event EventPossess
  (params (PossessedPawn :type Pawn%20Object%20Reference))
  (AI|RunBehaviorTree "/Game/Blueprints/Cockroach/BT_Cockroach.BT_Cockroach"))

(fn ConstructionScript)