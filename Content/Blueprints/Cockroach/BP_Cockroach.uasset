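; BP_Cockroach is a cockroach AI pawn that relays cloud hazard contact to its behavior through the blackboard.
; HandleCloudOverlap sets an InCloudDanger flag and stores the overlapping cloud's location in CloudLocation on the controller's blackboard.
; HandleCloudEnd clears the danger flag, leaving the stored location in place.
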(fn ConstructionScript)

(fn HandleCloudOverlap
  (params (Cloud :type BP%20Spray%20Cloud%20Object%20Reference))
  (bind _returnvalue (Pawn|GetController))
  (bind _returnvalue_2 (AI|GetBlackboard _returnvalue))
  (AI|Components|Blackboard|SetValueasBool _returnvalue_2 (Variables|Default|GetInCloudDanger) true)
  (AI|Components|Blackboard|SetValueasVector _returnvalue_2 (Variables|Default|GetCloudLocation) (Transformation|GetActorLocation Cloud)))

(fn HandleCloudEnd
  (AI|Components|Blackboard|SetValueasBool (AI|GetBlackboard (Pawn|GetController)) (Variables|Default|GetInCloudDanger) false))