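; BP_SprayCan is a usable spray can that spawns a spray cloud in front of the player.
; SprayCloud places a BP_SprayCloud actor a short distance along the player's forward vector, then disables further use.
; A timer event re-enables the can after a five-second cooldown.
; GetGripPoint exposes the can's GripPoint.
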(event Custom|SprayCloud
  (params (Player :type BP%20Player%20Object%20Reference))
  (if (Variables|Default|GetCanUse)
    (Game|SpawnActorfromClass "/Game/Blueprints/Cockroach/Spray/BP_SprayCloud.BP_SprayCloud_C" (Math|Transform|MakeTransform (+ (Transformation|GetActorLocation Player) (* (Transformation|GetActorForwardVector Player) 2e+02)) "0, 0, 0" "1.000000,1.000000,1.000000") "Undefined" "MultiplyWithRoot" 0 0)
    (Variables|Default|SetCanUse false)
    (Utilities|Time|SetTimerbyEvent (delegate Custom|Cooldown) 5.0)))

(event Custom|Cooldown
  (Variables|Default|SetCanUse true))

(fn ConstructionScript)

(fn GetGripPoint
  (return (Variables|Default|GetGripPoint)))