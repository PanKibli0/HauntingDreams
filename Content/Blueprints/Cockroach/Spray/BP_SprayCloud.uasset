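; BP_SprayCloud is a short-lived spray cloud actor that affects the player and cockroaches on overlap.
; It destroys itself through a timer set to a random few seconds at BeginPlay.
; An overlapping BP_Player receives a poison effect, while a BP_Cockroach is notified when it enters and leaves, leaving the cockroach's reaction to its own Blueprint.
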(event Custom|Stop
  (Actor|DestroyActor))

(event Collision|EventActorBeginOverlap
  (params (OtherActor :type Actor%20Object%20Reference))
  (bind _asbp_player (Utilities|Casting|CastToBP_Player OtherActor)
    (:then
      (Default|ApplyPoisonEff _asbp_player 6.0))
    (:CastFailed
      (bind _asbp_cockroach (Utilities|Casting|CastToBP_Cockroach OtherActor))
      (Default|HandleCloudOverlap _asbp_cockroach self))))

(event EventBeginPlay
  (Utilities|Time|SetTimerbyEvent (delegate Custom|Stop) (Math|Random|RandomFloatinRange 5.0 8.0)))

(event Collision|EventActorEndOverlap
  (params (OtherActor :type Actor%20Object%20Reference))
  (bind _asbp_cockroach (Utilities|Casting|CastToBP_Cockroach OtherActor))
  (Default|HandleCloudEnd _asbp_cockroach))

(fn ConstructionScript)