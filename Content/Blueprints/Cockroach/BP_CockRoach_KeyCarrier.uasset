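; Cockroach AI variant that carries a key, spawning a BP_Key attached to its KeyPoint on BeginPlay.
; A cloud overlap makes it drop the key onto the surface found by a downward trace, and its KeyCollision overlap reattaches the dropped key.
; Blackboard values track possession, carrier role and last drop location for the AI.
; The key's KeyPicked event clears the carrier flag and zeroes that location.
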(event OnComponentBeginOverlap(KeyCollision)
  (params (OverlappedComponent :type Primitive%20Component%20Object%20Reference) (OtherActor :type Actor%20Object%20Reference) (OtherComp :type Primitive%20Component%20Object%20Reference) (OtherBodyIndex :type Integer) (bFromSweep :type Boolean) (SweepResult :type Hit%20Result%20Structure%20%28by%20ref%29))
  (Utilities|Casting|CastToBP_Key OtherActor)
  (CallFunction|PickupKey))

(event Custom|KeyPicked
  (bind _returnvalue (AI|GetBlackboard 0))
  (AI|Components|Blackboard|SetValueasVector _returnvalue (Variables|Default|GetLastKeyDropLocation) "0, 0, 0")
  (AI|Components|Blackboard|SetValueasBool _returnvalue (Variables|Default|GetKeyCarrier) false))

(event EventBeginPlay
  (bind _returnvalue (Components|GetOwner))
  (bind _returnvalue_2 (AI|GetAIController _returnvalue))
  (bind _returnvalue_3 (AI|GetBlackboard _returnvalue_2))
  (Utilities|FlowControl|Sequence
    (:then_0
      (bind _returnvalue_4 (Game|SpawnActorfromClass "/Game/Blueprints/Enviroment/BP_Key.BP_Key_C" (Transformation|GetWorldTransform (Variables|Default|GetKeyPoint)) "AlwaysSpawn" "MultiplyWithRoot" 0 0))
      (bind _output_get (Variables|Default|SetHeldKey _returnvalue_4))
      (Collision|SetActorEnableCollision _output_get false)
      (Transformation|AttachComponentToComponent _output_get (Variables|Default|GetKeyPoint) "None" "SnapToTarget" "SnapToTarget" "KeepWorld" true)
      (Utilities|FlowControl|Delay 0.2)
      (AI|Components|Blackboard|SetValueasBool _returnvalue_3 (Variables|Default|GetHasKey) true)
      (AI|Components|Blackboard|SetValueasBool _returnvalue_3 (Variables|Default|GetKeyCarrier) true))
    (:then_1
      (EventDispatchers|BindEventtoKeyPicked _returnvalue_4 (delegate Custom|KeyPicked)))))

(fn ConstructionScript
  (|CallParentFunction))

(fn HandleCloudOverlap
  (params (Cloud :type BP%20Spray%20Cloud%20Object%20Reference))
  (CallFunction|DropKey)
  (|CallParentFunction Cloud))

(fn PickupKey
  (if (Utilities|IsValid (Variables|Default|GetDroppedKeyRef))
    (Transformation|AttachComponentToComponent (Variables|Default|GetDroppedKeyRef) (Variables|Default|GetKeyPoint) "None" "SnapToTarget" "SnapToTarget" "KeepWorld" true)
    (bind _output_get (Variables|Default|SetHeldKey (Variables|Default|GetDroppedKeyRef)))
    (Collision|SetActorEnableCollision _output_get false)
    (Variables|Default|SetDroppedKeyRef 0)
    (AI|Components|Blackboard|SetValueasBool (AI|GetBlackboard (Pawn|GetController)) (Variables|Default|GetHasKey) true)))

(fn DropKey
  (bind _returnvalue (Pawn|GetController))
  (bind _returnvalue_2 (AI|GetBlackboard _returnvalue))
  (if (Utilities|IsValid (Variables|Default|GetHeldKey))
    (bind (_outhit _returnvalue_3) (Collision|LineTraceByChannel (Transformation|GetActorLocation (Variables|Default|GetHeldKey)) (- (Transformation|GetActorLocation (Variables|Default|GetHeldKey)) "0.000000,0.000000,200.000000") "TraceTypeQuery1" false (Utilities|Array|MakeArray (Variables|Default|GetHeldKey)) "None"))
    (if _returnvalue_3
      (LocalVariables|SetDropLocation (+ (.ImpactPoint (Collision|BreakHitResult _outhit)) "0.000000,0.000000,10.000000"))
      (Transformation|DetachFromActor (Variables|Default|GetHeldKey) "KeepWorld" "KeepWorld" "KeepWorld")
      (Transformation|SetActorLocation (Variables|Default|GetHeldKey) (LocalVariables|GetDropLocation) false false)
      (Collision|SetActorEnableCollision (Variables|Default|GetHeldKey) true)
      (Variables|Default|SetDroppedKeyRef (Variables|Default|GetHeldKey))
      (AI|Components|Blackboard|SetValueasVector _returnvalue_2 (Variables|Default|GetLastKeyDropLocation) (LocalVariables|GetDropLocation))
      (Variables|Default|SetHeldKey 0)
      (AI|Components|Blackboard|SetValueasBool _returnvalue_2 (Variables|Default|GetHasKey) false)
      (Development|PrintString "DROP KEY")
      (else
        (return)))))