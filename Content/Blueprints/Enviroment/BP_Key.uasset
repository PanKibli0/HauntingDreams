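; BP_Key is a pickup key actor that the player collects through an Interact event on a component tagged "Key".
; On pickup it reports its TaskID as completed to the current loop held by BP_GameMode, then hides itself and disables collision.
; It then sets HasKey on BP_Player, prints a Polish "key found" message and calls KeyPicked.
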(event EventInteract
  (params (HitComponent :type Primitive%20Component%20Object%20Reference) (Location :type Vector :default "0, 0, 0") (HeldItem :type Actor%20Object%20Reference))
  (if (Components|ComponentHasTag HitComponent "Key")
    (bind _asbp_game_mode (Utilities|Casting|CastToBP_GameMode (Game|GetGameMode)))
    (Default|NotifyTaskCompleted (Variables|/Game/Player/BP_GameMode.BP_GameMode_C|GetCurrentLoopRef _asbp_game_mode) (Variables|Default|GetTaskID))
    (Rendering|SetActorHiddenInGame true)
    (Collision|SetActorEnableCollision false)
    (bind _asbp_player (Utilities|Casting|CastToBP_Player (Game|GetPlayerCharacter 0)))
    (Variables|/Game/Player/BP_Player.BP_Player_C|SetHasKey _asbp_player true)
    (Development|PrintString "Znaleziono klucz")
    (Default|CallKeyPicked)))

(fn ConstructionScript)