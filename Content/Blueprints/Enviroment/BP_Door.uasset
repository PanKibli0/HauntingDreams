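; BP_Door is a hinged door that toggles open and closed through its OpenDoor event, unless it is locked.
; A locked door only prints debug text, including a Polish "door locked" message.
; Otherwise it flips IsOpened and plays or reverses a timeline that lerps the Door component's yaw through a quarter turn.
; A separate CloseDoor event always clears IsOpened and reverses the timeline, without checking the lock.
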(event Custom|OpenDoor
  (bind _islocked (Variables|Default|GetisLocked))
  (Development|PrintString "Hello" _islocked)
  (if _islocked
    (Development|PrintString "ZAMKNIĘTE DRZWI")
    (elif (Variables|Default|GetisOpened)
      (Variables|Default|SetisOpened false)
      (bind _opening (Timeline|TL_OpenDoor ReverseFromEnd)
        (:Update
          (Transformation|SetRelativeRotation (Variables|Default|GetDoor) (Math|Rotator|MakeRotator 0.0 0.0 (Math|Float|Lerp 0.0 9e+01 _opening)) false false)))
      (else
        (Variables|Default|SetisOpened true)
        (Timeline|TL_OpenDoor PlayFromStart)))))

(event Custom|CloseDoor
  (Variables|Default|SetisOpened false)
  (bind _opening (Timeline|TL_OpenDoor ReverseFromEnd)
    (:Update
      (Transformation|SetRelativeRotation (Variables|Default|GetDoor) (Math|Rotator|MakeRotator 0.0 0.0 (Math|Float|Lerp 0.0 9e+01 _opening)) false false))))

(fn ConstructionScript)