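; Inspectable world item that the player can pull up in front of them and rotate with the mouse, with input enabled only while overlapping its collision.
; Interact, gated by a DoOnce, locks movement and look, shows the cursor and runs a timeline lerping the item to the player's Item component transform.
; Q resets the gate, restores controls and reverses the timeline to return the item to its original transform.
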(event OnComponentBeginOverlap(collision)
  (params (OverlappedComponent :type Primitive%20Component%20Object%20Reference) (OtherActor :type Actor%20Object%20Reference) (OtherComp :type Primitive%20Component%20Object%20Reference) (OtherBodyIndex :type Integer) (bFromSweep :type Boolean) (SweepResult :type Hit%20Result%20Structure%20%28by%20ref%29))
  (Input|EnableInput (Game|GetPlayerController 0)))

(event OnComponentEndOverlap(collision)
  (params (OverlappedComponent :type Primitive%20Component%20Object%20Reference) (OtherActor :type Actor%20Object%20Reference) (OtherComp :type Primitive%20Component%20Object%20Reference) (OtherBodyIndex :type Integer))
  (Input|DisableInput (Game|GetPlayerController 0)))

(event EventBeginPlay
  (bind _item (Variables|Default|Getitem))
  (bind _output_get (Variables|Default|SetOriginalLocation (Transformation|GetWorldLocation _item)))
  (bind _output_get_2 (Variables|Default|SetOriginalRotation (Transformation|GetWorldRotation _item))))

(event EventInteract
  (params (HitComponent :type Primitive%20Component%20Object%20Reference) (Location :type Vector :default "0, 0, 0") (HeldItem :type Actor%20Object%20Reference))
  (Utilities|FlowControl|DoOnce false
    (:Completed
      (Variables|/Script/Engine.PlayerController|SetbShowMouseCursor (Game|GetPlayerController 0) true)
      (Variables|Default|SetcanInspect true)
      (bind _asbp_player (Utilities|Casting|CastToBP_Player (Game|GetPlayerCharacter 0)))
      (Pawn|Components|CharacterMovement|DisableMovement (Variables|/Script/Engine.Character|GetCharacterMovement (Game|GetPlayerCharacter 0)))
      (Input|SetIgnoreLookInput (Game|GetPlayerController 0) true)
      (bind _track (Timeline|Timeline PlayFromStart)
        (:Update
          (Transformation|SetWorldTransform (Variables|Default|Getitem) (Math|Transform|MakeTransform (Math|Vector|Lerp(Vector) (stale EventBeginPlay _output_get) (.location (Transformation|GetWorldTransform (Variables|/Game/Player/BP_Player.BP_Player_C|Getitem _asbp_player))) _track) (Math|Rotator|Lerp(Rotator) (stale EventBeginPlay _output_get_2) (.rotation (Transformation|GetWorldTransform (Variables|/Game/Player/BP_Player.BP_Player_C|Getitem _asbp_player))) _track) "1.000000,1.000000,1.000000") false false))))))

(event EventTick
  (params (DeltaSeconds :type Float%20%28single-precision%29))
  (if (Variables|Default|GetcanInspect)
    (Transformation|AddLocalRotation (Variables|Default|Getitem) (Math|Rotator|MakeRotator (* (stale Input|MouseEvents|MouseX AxisValue) 0.5) (* (stale Input|MouseEvents|MouseY AxisValue) -0.5) 0.0) false false)))

(event Input|MouseEvents|MouseX
  (params (AxisValue :type Float%20%28single-precision%29))
  (if (Variables|Default|GetcanInspect)
    (Transformation|AddLocalRotation (Variables|Default|Getitem) (Math|Rotator|MakeRotator (* AxisValue 0.5) (* (stale Input|MouseEvents|MouseY AxisValue) -0.5) 0.0) false false)))

(event Input|MouseEvents|MouseY
  (params (AxisValue :type Float%20%28single-precision%29))
  (if (Variables|Default|GetcanInspect)
    (Transformation|AddLocalRotation (Variables|Default|Getitem) (Math|Rotator|MakeRotator (* (stale Input|MouseEvents|MouseX AxisValue) 0.5) (* AxisValue -0.5) 0.0) false false)))

(event Input|KeyboardEvents|Q
  (params (Key :type Key%20Structure :default "None"))
  (bind _returnvalue (Game|GetPlayerController 0))
  (:Pressed
    (Utilities|FlowControl|Sequence
      (:then_0
        (Utilities|FlowControl|DoOnce false) ; enters at Reset
      )
      (:then_1
        (Variables|Default|SetcanInspect false)
        (Pawn|Components|CharacterMovement|SetMovementMode (Variables|/Script/Engine.Character|GetCharacterMovement (Game|GetPlayerCharacter 0)) "MOVE_Walking" 0)
        (Variables|/Script/Engine.PlayerController|SetbShowMouseCursor _returnvalue false)
        (Input|ResetIgnoreLookInput _returnvalue)
        (Input|SetInputModeGameOnly _returnvalue false)
        (bind _track (Timeline|Timeline Reverse)
          (:Update
            (Transformation|SetWorldTransform (Variables|Default|Getitem) (Math|Transform|MakeTransform (Math|Vector|Lerp(Vector) (stale EventBeginPlay _output_get) (.location (Transformation|GetWorldTransform (Variables|/Game/Player/BP_Player.BP_Player_C|Getitem (stale EventInteract _asbp_player)))) _track) (Math|Rotator|Lerp(Rotator) (stale EventBeginPlay _output_get_2) (.rotation (Transformation|GetWorldTransform (Variables|/Game/Player/BP_Player.BP_Player_C|Getitem (stale EventInteract _asbp_player)))) _track) "1.000000,1.000000,1.000000") false false)))))))

(fn ConstructionScript)