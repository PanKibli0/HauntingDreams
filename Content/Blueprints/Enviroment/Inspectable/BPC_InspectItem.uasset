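; Actor component that lets the player inspect its owning item up close and rotate it with the mouse.
; Interact toggles inspection through a FlipFlop, locking the player's movement and look while showing the cursor, then restoring them.
; Tick eases the owner toward the inspect Location and applies mouse-delta rotation, or eases it back to its BeginPlay position while snapping to its original rotation.
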(event EventBeginPlay
  (bind _returnvalue (Components|GetOwner))
  (bind _output_get (Variables|Default|SetOriginalLocation (Transformation|GetActorLocation _returnvalue)))
  (Variables|Default|SetOriginalRotation (Transformation|GetActorRotation _returnvalue)))

(event EventInteract
  (params (HitComponent :type Primitive%20Component%20Object%20Reference) (Location :type Vector :default "0, 0, 0") (HeldItem :type Actor%20Object%20Reference))
  (bind _returnvalue (Game|GetPlayerCharacter 0))
  (bind _returnvalue_2 (Game|GetPlayerController 0))
  (bind _returnvalue_3 (Components|GetOwner))
  (bind _isa (Utilities|FlowControl|FlipFlop)
    (:A
      (Variables|Default|SetisInspecting _isa)
      (Input|EnableInput (Components|GetOwner) _returnvalue_2)
      (Variables|/Script/Engine.PlayerController|SetbShowMouseCursor (Game|GetPlayerController 0) true)
      (Variables|Default|SetcanInspect true)
      (Utilities|Casting|CastToBP_Player _returnvalue)
      (Pawn|Components|CharacterMovement|DisableMovement (Variables|/Script/Engine.Character|GetCharacterMovement _returnvalue))
      (Input|SetIgnoreLookInput (Game|GetPlayerController 0) true))
    (:B
      (Variables|Default|SetisInspecting false)
      (Pawn|Components|CharacterMovement|SetMovementMode (Variables|/Script/Engine.Character|GetCharacterMovement (Game|GetPlayerCharacter 0)) "MOVE_Walking" 0)
      (Variables|/Script/Engine.PlayerController|SetbShowMouseCursor _returnvalue_2 false)
      (Input|ResetIgnoreLookInput _returnvalue_2)
      (Input|SetInputModeGameOnly _returnvalue_2 false)
      (Input|DisableInput _returnvalue_3 _returnvalue_2)
      (Transformation|DetachFromActor _returnvalue_3 "KeepWorld" "KeepWorld" "KeepWorld"))))

(event EventTick
  (params (DeltaSeconds :type Float%20%28single-precision%29))
  (bind _returnvalue (Components|GetOwner))
  (bind _returnvalue_2 (Game|GetPlayerController 0))
  (bind _returnvalue_3 (Transformation|GetActorLocation _returnvalue))
  (bind (_deltax _deltay) (Class|PlayerController|GetInputMouseDelta _returnvalue_2))
  (if (Variables|Default|GetisInspecting)
    (Transformation|SetActorLocation _returnvalue (Math|Interpolation|VInterpTo _returnvalue_3 (stale EventInteract Location) DeltaSeconds 2.0) false false)
    (Transformation|AddActorLocalRotation (Components|GetOwner) (Math|Rotator|MakeRotator (* _deltax 1.2) (* _deltay -1.2) 0.0) false false)
    (else
      (Transformation|SetActorLocationAndRotation _returnvalue (Math|Interpolation|VInterpTo _returnvalue_3 (stale EventBeginPlay _output_get) DeltaSeconds 2.0) (Variables|Default|GetOriginalRotation)))))