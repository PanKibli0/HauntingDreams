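; Actor component that places the current loop's props on its owning actor, drawing them from an object pool in BP_GameMode.
; On BeginPlay it reads PropsToSpawn from the game mode's current LoopSequence entry and matches each tag to the owner's first scene component with that tag.
; Each pooled prop snaps to that component's location and rotation, keeping world scale, and is tracked in ActiveProps.
; ClearProps returns tracked props to the pool and empties the list.
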(event EventBeginPlay
  (bind _asbp_game_mode (Utilities|Casting|CastToBP_GameMode (Game|GetGameMode)))
  (for _array_element (Variables|/Game/DataAssets/PDA_LoopConfig.PDA_LoopConfig_C|GetPropsToSpawn (Utilities|Array|Get(acopy) (Variables|/Game/Player/BP_GameMode.BP_GameMode_C|GetLoopSequence _asbp_game_mode) (Variables|/Game/Player/BP_GameMode.BP_GameMode_C|GetCurrentLoopIndex _asbp_game_mode)))
    (Utilities|IsValid (Utilities|Array|Get(acopy) (Variables|/Game/Player/BP_GameMode.BP_GameMode_C|GetLoopSequence _asbp_game_mode) (Variables|/Game/Player/BP_GameMode.BP_GameMode_C|GetCurrentLoopIndex _asbp_game_mode))
      (:Is%20Valid
        (if (> (Utilities|Array|Length (Actor|GetComponentsbyTag (Components|GetOwner) "/Script/Engine.SceneComponent" (.Tag (Utilities|Struct|BreakS_PropSpawn _array_element)))) 0)
          (bind _spawnedprop (Default|GetPropfromPool _asbp_game_mode (.PropClass (Utilities|Struct|BreakS_PropSpawn _array_element)) (Transformation|GetWorldTransform (Utilities|Array|Get(acopy) (Actor|GetComponentsbyTag (Components|GetOwner) "/Script/Engine.SceneComponent" (.Tag (Utilities|Struct|BreakS_PropSpawn _array_element)))))))
          (Utilities|IsValid _spawnedprop
            (:Is%20Valid
              (Utilities|Array|Add (Variables|Default|GetActiveProps) _spawnedprop)
              (Transformation|AttachComponentToComponent _spawnedprop (Utilities|Array|Get(acopy) (Actor|GetComponentsbyTag (Components|GetOwner) "/Script/Engine.SceneComponent" (.Tag (Utilities|Struct|BreakS_PropSpawn _array_element)))) "None" "SnapToTarget" "SnapToTarget" "KeepWorld" true))))))))

(fn ClearProps
  (for _array_element (Variables|Default|GetActiveProps)
    (Utilities|IsValid _array_element
      (:Is%20Valid
        (bind _asbp_game_mode (Utilities|Casting|CastToBP_GameMode (Game|GetGameMode)))
        (Default|ReturnProptoPool _asbp_game_mode _array_element))))
  (Utilities|Array|Clear (Variables|Default|GetActiveProps)))