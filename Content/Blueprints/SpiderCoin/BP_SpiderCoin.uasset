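; BP_SpiderCoin is an AI-controlled spider that reacts to being lit, feeding light events into its behavior logic.
; It registers with the level's BP_LightSpiderManager on BeginPlay and unregisters on EndPlay.
; OnSeenByLight and OnLostLight toggle the IsLit key on the AI controller's blackboard, and being seen also stores the LightHitLocation.
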(event Custom|OnSeenByLight
  (params (HitLocation :type Vector))
  (bind _asaicontroller (Utilities|Casting|CastToAIController (Pawn|GetController)))
  (AI|Components|Blackboard|SetValueasBool (AI|GetBlackboard _asaicontroller) (Variables|Default|GetIsLit) true)
  (AI|Components|Blackboard|SetValueasVector (AI|GetBlackboard _asaicontroller) (Variables|Default|GetLightHitLocation) HitLocation))

(event Custom|OnLostLight
  (bind _asaicontroller (Utilities|Casting|CastToAIController (Pawn|GetController)))
  (AI|Components|Blackboard|SetValueasBool (AI|GetBlackboard _asaicontroller) (Variables|Default|GetIsLit) false))

(event EventEndPlay
  (params (EndPlayReason :type EEndPlayReason%20Enum :default "Destroyed"))
  (bind _returnvalue (Actor|GetActorOfClass "/Game/Blueprints/SpiderCoin/BP_LightSpiderManager.BP_LightSpiderManager_C"))
  (Default|UnregisterSpider _returnvalue self))

(event EventBeginPlay
  (bind _returnvalue (Actor|GetActorOfClass "/Game/Blueprints/SpiderCoin/BP_LightSpiderManager.BP_LightSpiderManager_C"))
  (Default|RegisterSpider _returnvalue self))

(fn ConstructionScript)