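; Manager actor that tells registered coin spiders whether the player's flashlight is lighting them.
; A looping timer tests each spider against the spotlight's attenuation radius and outer cone angle, then line-traces for occlusion.
; Lit spiders receive OnSeenByLight with the hit location of the beam's forward trace; others, or all when the light is hidden, receive OnLostLight.
; Spiders enter and leave the list through RegisterSpider and UnregisterSpider.
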(event Custom|CheckSpiders
  (bind _flashlightref (Variables|Default|GetFlashlightRef))
  (bind _returnvalue (Transformation|GetWorldLocation _flashlightref))
  (Utilities|IsValid (Variables|Default|GetFlashlightRef)
    (:Is%20Valid
      (if (Rendering|IsVisible (Variables|Default|GetFlashlightRef))
        (bind _outhit (Collision|LineTraceByChannel _returnvalue (+ _returnvalue (* (Math|Vector|GetForwardVector (Variables|Default|GetFlashlightRef)) (Variables|/Script/Engine.LocalLightComponent|GetAttenuationRadius (Variables|Default|GetFlashlightRef)))) "TraceTypeQuery1" false 0 "None"))
        (for _array_element (Variables|Default|GetRegisteredSpidersCoin)
          (if (<= (Math|Vector|VectorLength (- (Transformation|GetActorLocation _array_element) (Transformation|GetWorldLocation (Variables|Default|GetFlashlightRef)))) (Variables|/Script/Engine.LocalLightComponent|GetAttenuationRadius (Variables|Default|GetFlashlightRef))) ; Distance
            (if (>= (Math|Vector|DotProduct (Math|Vector|Normalize (- (Transformation|GetActorLocation _array_element) (Transformation|GetWorldLocation (Variables|Default|GetFlashlightRef)))) (Math|Vector|GetForwardVector (Variables|Default|GetFlashlightRef))) (Math|Trig|Cos(Radians) (Math|Trig|DegreesToRadians (Variables|/Script/Engine.SpotLightComponent|GetOuterConeAngle (Variables|Default|GetFlashlightRef))))) ; Angle
              (bind _returnvalue_2 (Collision|LineTraceByChannel (Transformation|GetWorldLocation (Variables|Default|GetFlashlightRef)) (Transformation|GetActorLocation _array_element) "TraceTypeQuery1" false (Utilities|Array|MakeArray _array_element) "None"))
              (if _returnvalue_2
                (Default|OnLostLight _array_element)
                (else
                  (Default|OnSeenbyLight _array_element (.Location (Collision|BreakHitResult _outhit)))))
              (else
                (Default|OnLostLight _array_element)))
            (else
              (Default|OnLostLight _array_element))))
        (else
          (for _array_element_2 (Variables|Default|GetRegisteredSpidersCoin)
            (Default|OnLostLight _array_element_2)))))))

(event EventBeginPlay
  (bind _asbp_player (Utilities|Casting|CastToBP_Player (Game|GetPlayerCharacter 0)))
  (Variables|Default|SetFlashlightRef (Actor|GetComponentbyClass _asbp_player "/Script/Engine.SpotLightComponent"))
  (Utilities|Time|SetTimerbyEvent (delegate Custom|CheckSpiders) 0.2 true))

(fn ConstructionScript)

(fn UnregisterSpider
  (params (SpiderRef :type BP%20Spider%20Coin%20Object%20Reference))
  (Utilities|Array|RemoveItem (Variables|Default|GetRegisteredSpidersCoin) SpiderRef))

(fn RegisterSpider
  (params (SpiderRef :type BP%20Spider%20Coin%20Object%20Reference))
  (Utilities|Array|AddUnique (Variables|Default|GetRegisteredSpidersCoin) SpiderRef))