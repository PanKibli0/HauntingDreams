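; BP_Loop is a self-chaining house segment that forms an endless loop of spaces for the player.
; When the player's pawn first enters its Box trigger, it closes its child-actor BP_Door and spawns another BP_Loop at the Arrow, offset in height and rotation.
; Each new segment keeps a PrevLoop reference to its spawner, and the triggered segment destroys its predecessor after a short delay.
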(event OnComponentBeginOverlap(Box)
  (params (OverlappedComponent :type Primitive%20Component%20Object%20Reference) (OtherActor :type Actor%20Object%20Reference) (OtherComp :type Primitive%20Component%20Object%20Reference) (OtherBodyIndex :type Integer) (bFromSweep :type Boolean) (SweepResult :type Hit%20Result%20Structure%20%28by%20ref%29))
  (bind _arrow (Variables|Default|GetArrow))
  (bind _returnvalue (Transformation|GetWorldTransform _arrow))
  (if (and (== OtherActor (Pawn|GetControlledPawn (Game|GetPlayerController 0))) (not (Variables|Default|GetbeenTriggered)))
    (Variables|Default|SetbeenTriggered true)
    (Default|CloseDoor (Variables|Default|GetDoorRef))
    (Utilities|FlowControl|Sequence
      (:then_0
        (Utilities|IsValid (Variables|Default|GetPrevLoop)
          (:Is%20Valid
            (Utilities|FlowControl|Delay 2.0)
            (Actor|DestroyActor (Variables|Default|GetPrevLoop)))))
      (:then_1
        (bind _returnvalue_2 (Game|SpawnActorfromClass "BP_Loop_C" (Math|Transform|MakeTransform (Math|Vector|MakeVector (.x (.location _returnvalue)) (.y (.location _returnvalue)) (+ (.z (.location _returnvalue)) 156.0)) (Math|Rotator|CombineRotators (.rotation _returnvalue) "0.000000,-90.000000,0.000000") "1.000000,1.000000,1.000000") "AlwaysSpawn" "MultiplyWithRoot" 0 0))
        (Variables|BP_Loop_C|SetPrevLoop _returnvalue_2 self)))))

(event EventBeginPlay
  (bind _asbp_door (Utilities|Casting|CastToBP_Door (Variables|/Script/Engine.ChildActorComponent|GetChildActor (Variables|Default|GetDoor))))
  (Variables|Default|SetDoorRef _asbp_door))

(fn ConstructionScript)