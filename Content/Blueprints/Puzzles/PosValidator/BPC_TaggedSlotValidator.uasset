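; Puzzle validator component that checks whether every slot holds an item whose tag matches the tag that slot accepts.
; When an item is placed, it waits until all slots are occupied, then compares tags slot by slot via message calls.
; The first mismatch or invalid item increments a fail count and calls puzzle failed.
; A full match latches the solved state and calls puzzle solved; item removal does nothing.
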(fn CheckSolved
  (for _array_element (Variables|Default|GetSlots)
    (bind _currentitem (Default|GetCurrentItem _array_element))
    (Utilities|IsValid _currentitem
      (:Is%20Valid
        (bind _itemtag (Class|BPITaggable|GetItemTag(Message) _currentitem))
        (bind _acceptedtag (Class|BPIValidatorSlot|GetAcceptedTag(Message) (Utilities|ToObject(Interface) _array_element)))
        (if (not (== _itemtag _acceptedtag))
          (Math|Integer|IncrementInt (Variables|Default|GetFailCount) :!label _label
            (:%20%20
              (Default|CallOnPuzzleFailed)
              (return)))))
      (:Is%20Not%20Valid
        (goto _label))))
  (Variables|Default|SetAlreadySolved true)
  (Default|CallOnPuzzleSolved))

(fn AreAllSlotsOccupied
  (for _array_element (Variables|Default|GetSlots)
    (Development|PrintString (Utilities|GetDisplayName (Utilities|ToObject(Interface) _array_element)))
    (bind _isoccupied (Class|BPIValidatorSlot|IsOccupied(Message) (Utilities|ToObject(Interface) _array_element)))
    (if (not _isoccupied)
      (return false)))
  (return true))

(fn OnItemPlaced
  (params (Item :type Actor%20Object%20Reference) (Slot :type Actor%20Object%20Reference))
  (bind _all_occupied (CallFunction|AreAllSlotsOccupied))
  (if (and _all_occupied (not (Variables|Default|GetAlreadySolved)))
    (CallFunction|CheckSolved)))

(fn OnItemRemoved
  (params (Item :type Actor%20Object%20Reference) (Slot :type Actor%20Object%20Reference)))

(fn Fail)