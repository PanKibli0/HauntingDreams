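; Base puzzle validator component that decides whether a slot-based puzzle is solved once every slot holds an item.
; On item placement it polls each slot for occupancy through interface messages, then runs CheckSolved, a stub returning false for child validators to override.
; The result fires the solved or failed dispatcher with a debug print, latching success and counting failures; item removal does nothing.
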(fn CheckSolved
  (return false))

(fn AreAllSlotsOccupied
  (for _array_element (Variables|Default|GetSlots)
    (bind _isoccupied (Class|BPIValidatorSlot|IsOccupied(Message) (Utilities|ToObject(Interface) _array_element)))
    (if (not _isoccupied)
      (return false)))
  (return true))

(fn OnItemPlaced
  (params (Item :type Actor%20Object%20Reference) (Slot :type Actor%20Object%20Reference))
  (bind _all_occupied (CallFunction|AreAllSlotsOccupied))
  (if (and _all_occupied (not (Variables|Default|GetAlreadySolved)))
    (bind _issolved (CallFunction|CheckSolved))
    (if _issolved
      (Variables|Default|SetAlreadySolved true)
      (Default|CallOnPuzzleSolved)
      (Development|PrintString "PUZZLE SOLVED" true true "(R=1.000000,G=0.860859,B=0.000000,A=1.000000)")
      (else
        (Math|Integer|IncrementInt (Variables|Default|GetFailCount)
          (:%20%20
            (Default|CallOnPuzzleFailed)
            (Development|PrintString "PUZZLE FAILED" true true "(R=1.000000,G=0.169378,B=0.023568,A=1.000000)")))))))

(fn OnItemRemoved
  (params (Item :type Actor%20Object%20Reference) (Slot :type Actor%20Object%20Reference)))