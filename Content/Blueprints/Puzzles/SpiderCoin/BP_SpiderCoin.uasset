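; BP_SpiderCoin is an AI-controlled puzzle spider that reacts to light and dies after enough continuous exposure.
; Each seen-by-light event writes the lit flag and hit location to the AI Blackboard and adds a fixed tick interval to the exposure timer, with debug prints.
; At the death threshold it calls SpiderDeath and destroys itself, while losing the light clears the flag and resets the timer.
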(event Custom|OnSeenByLight
  (params (HitLocation :type Vector))
  (bind _asaicontroller (Utilities|Casting|CastToAIController (Pawn|GetController)))
  (AI|Components|Blackboard|SetValueasBool (AI|GetBlackboard _asaicontroller) (Variables|Default|GetIsLit) true)
  (AI|Components|Blackboard|SetValueasVector (AI|GetBlackboard _asaicontroller) (Variables|Default|GetLightHitLocation) HitLocation)
  (bind _output_get (Variables|Default|SetLightExposureTime (+ (Variables|Default|GetLightExposureTime) (Variables|Default|GetExposureTickInterval))))
  (Development|PrintString (Utilities|String|Append "SPIDER TIME: " (Utilities|String|ToString(Float) _output_get)) true true "(R=1.000000,G=0.810097,B=0.000000,A=1.000000)")
  (if (>= _output_get (Variables|Default|GetTimeToDie))
    (Development|PrintString "SPIDER DIE")
    (Default|CallSpiderDeath self)
    (Actor|DestroyActor)))

(event Custom|OnLostLight
  (bind _asaicontroller (Utilities|Casting|CastToAIController (Pawn|GetController)))
  (AI|Components|Blackboard|SetValueasBool (AI|GetBlackboard _asaicontroller) (Variables|Default|GetIsLit) false)
  (Variables|Default|SetLightExposureTime 0.0))

(fn ConstructionScript)