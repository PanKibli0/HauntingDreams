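; Blueprint function library for puzzles with a helper that finds an unobstructed random spawn point inside a box component.
; FindValidSpawnPoint uses capped rejection sampling, picking random points in the box's scaled extent and box-overlapping each against the given object types, minus ignored actors.
; It returns a success flag and the last candidate, which may be blocked on failure, and prints each overlap count for debugging.
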(fn FindValidSpawnPoint
  (params (SpawnArea :type Box%20Component%20Object%20Reference) (CheckExtent :type Vector) (ObjectTypesToCheck :type Array%20of%20EObjectTypeQuery%20Enums :default "ObjectTypeQuery1") (ActorsToIgnore :type Array%20of%20Actor%20Object%20References))
  (LocalVariables|SetAttempts 0)
  (LocalVariables|SetFoundStopLocal false)
  (while (and (< (LocalVariables|GetAttempts) 10) (not (LocalVariables|GetFoundStopLocal)))
    (bind _output_get (LocalVariables|SetCandidateLocation (Math|Random|RandomPointinBoundingBox (Transformation|GetWorldLocation SpawnArea) (Components|Box|GetScaledBoxExtent SpawnArea))))
    (bind _outactors (Collision|BoxOverlapActors 0 _output_get CheckExtent ObjectTypesToCheck 0 ActorsToIgnore :!class /Script/Engine.KismetSystemLibrary))
    (Development|PrintString 0 (Utilities|String|ToString(Integer) (Utilities|Array|Length _outactors)))
    (LocalVariables|SetFoundStopLocal (== (Utilities|Array|Length _outactors) 0))
    (Math|Integer|IncrementInt (LocalVariables|GetAttempts)))
  (return (LocalVariables|GetFoundStopLocal) (LocalVariables|GetCandidateLocation)))