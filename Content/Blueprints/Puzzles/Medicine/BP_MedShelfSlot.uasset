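; Medicine shelf puzzle slot that holds one item and registers itself with the parent actor's BPC_TaggedSlotValidator on BeginPlay.
; TryHold places, takes or swaps the held item, accepting anything under the Item.med tag and returning what the caller should now hold.
; Placing moves the item to the slot and makes it visible; placements and removals notify the validator, with ExpectedTag exposed through a getter.
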(event EventBeginPlay
  (bind _returnvalue (Actor|GetAttachParentActor))
  (bind _returnvalue_2 (Actor|GetComponentbyClass _returnvalue "/Game/Blueprints/Puzzles/PosValidator/BPC_TaggedSlotValidator.BPC_TaggedSlotValidator_C"))
  (Utilities|IsValid _returnvalue
    (:Is%20Valid
      (Utilities|IsValid _returnvalue_2
        (:Is%20Valid
          (Utilities|Array|AddUnique (Variables|/Game/Blueprints/Puzzles/PosValidator/BPC_TaggedSlotValidator.BPC_TaggedSlotValidator_C|GetSlots _returnvalue_2) self))))))

(fn ConstructionScript)

(fn PlaceItem
  (params (Item :type Actor%20Object%20Reference))
  (bind _output_get (Variables|Default|SetCurrentItem Item))
  ;[0.15 0.15 0.15 0.5] dopasowac rotate nw do czego tak na serio
  (Transformation|SetActorLocationAndRotation _output_get (Transformation|GetActorLocation))
  (Rendering|SetVisibility (Actor|GetComponentbyClass _output_get "/Script/Engine.StaticMeshComponent") true true)
  (Default|OnItemPlaced (Actor|GetComponentbyClass (Actor|GetAttachParentActor) "/Game/Blueprints/Puzzles/PosValidator/BPC_TaggedSlotValidator.BPC_TaggedSlotValidator_C") Item self))

(fn RemoveItem
  (Default|OnItemRemoved (Actor|GetComponentbyClass (Actor|GetAttachParentActor) "/Game/Blueprints/Puzzles/PosValidator/BPC_TaggedSlotValidator.BPC_TaggedSlotValidator_C") (Variables|Default|GetCurrentItem) self)
  (Variables|Default|SetCurrentItem 0))

(fn GetAcceptedTag
  (return (Variables|Default|GetExpectedTag)))

(fn GetCurrentItem
  (return (Variables|Default|GetCurrentItem)))

(fn GetSlotIndex
  (return (Variables|Default|GetSlotIndex)))

(fn IsOccupied
  (return (Utilities|IsValid (Variables|Default|GetCurrentItem))))

(fn TryHold
  (params (Held%20Item :type Actor%20Object%20Reference))
  (bind _isoccupied (CallFunction|IsOccupied))
  (if _isoccupied
    (Utilities|IsValid Held%20Item
      (:Is%20Valid
        (bind _itemtag (Class|BPITaggable|GetItemTag(Message) Held%20Item))
        (if (GameplayTags|MatchesTag _itemtag "(TagName=\"Item.med\")")
          (LocalVariables|SetOccupiedItem (Variables|Default|GetCurrentItem))
          (CallFunction|RemoveItem)
          (CallFunction|PlaceItem Held%20Item)
          (return (LocalVariables|GetOccupiedItem))
          (else
            (return Held%20Item))))
      (:Is%20Not%20Valid
        (LocalVariables|SetOccupiedItem (Variables|Default|GetCurrentItem))
        (CallFunction|RemoveItem)
        (return (LocalVariables|GetOccupiedItem))))
    (else
      (Utilities|IsValid Held%20Item
        (:Is%20Valid
          (bind _itemtag_2 (Class|BPITaggable|GetItemTag(Message) Held%20Item))
          (if (GameplayTags|MatchesTag _itemtag_2 "(TagName=\"Item.med\")")
            (CallFunction|PlaceItem Held%20Item)
            (return 0)
            (else
              (return Held%20Item))))
        (:Is%20Not%20Valid
          (return 0))))))