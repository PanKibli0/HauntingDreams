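; BP_Dust is a sweepable dust patch for the dust sweeping puzzle.
; On BeginPlay it randomizes its XY scale, yaw and the dark base color of a dynamic M_Dust material on its plane.
; Interacting while holding a BP_Broom fires the Sweeped dispatcher with itself, then destroys the actor.
; Adding it to a puzzle collection is only a debug print placeholder.
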(event EventInteract
  (params (HitComponent :type Primitive%20Component%20Object%20Reference) (Location :type Vector :default "0, 0, 0") (HeldItem :type Actor%20Object%20Reference))
  (Utilities|Casting|CastToBP_Broom HeldItem)
  (Default|CallSweeped self)
  (Actor|DestroyActor))

(event EventBeginPlay
  (bind _returnvalue (Math|Random|RandomFloatinRange 0.05 0.35))
  (Transformation|SetActorScale3D (Math|Vector|MakeVector (Math|Random|RandomFloatinRange 0.5 1.2) (Math|Random|RandomFloatinRange 0.5 1.2) 1.0))
  (Transformation|SetActorRotation (Math|Rotator|MakeRotator 0.0 0.0 (Math|Random|RandomFloatinRange 0.0 3.6e+02)))
  (bind _returnvalue_2 (Rendering|Material|CreateDynamicMaterialInstance (Variables|Default|GetPlane) 0 "/Game/Blueprints/Puzzles/DustSweeping/M_Dust.M_Dust" "None" :!class /Script/Engine.PrimitiveComponent))
  (Rendering|Material|SetVectorParameterValue _returnvalue_2 "BaseColor" (Math|Color|MakeColor _returnvalue _returnvalue _returnvalue) :!class /Script/Engine.MaterialInstanceDynamic)
  (Development|PrintString "ADD TO PUZZLE COLLECTION" false false))

(fn ConstructionScript)