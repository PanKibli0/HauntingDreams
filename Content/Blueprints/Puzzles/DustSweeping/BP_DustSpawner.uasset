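; BP_DustSpawner scatters a random number of BP_Dust actors inside its SpawnArea box at BeginPlay for the dust sweeping puzzle.
; Each piece gets up to ten random candidate points, accepted only if a flat box overlap finds no world static or dynamic actors, and is skipped otherwise.
; Already spawned dust is ignored by that check, so pieces can overlap one another.
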(event EventBeginPlay
  (for _index (range 0 (Math|Random|RandomIntegerinRange 8 16))
    (Variables|Default|SetAttempts 0)
    (Variables|Default|SetFoundSpot false)
    (while (and (< (Variables|Default|GetAttempts) 10) (not (Variables|Default|GetFoundSpot)))
      (bind _output_get (Variables|Default|SetCandidateLocation (Math|Random|RandomPointinBoundingBox (Transformation|GetActorLocation) (Components|Box|GetScaledBoxExtent (Variables|Default|GetSpawnArea)))))
      (bind _outactors (Collision|BoxOverlapActors _output_get "15.000000,15.000000,0.000000" (Utilities|Array|MakeArray "ObjectTypeQuery1" "ObjectTypeQuery2") 0 (Variables|Default|GetSpawnedDust) :!class /Script/Engine.KismetSystemLibrary))
      (Variables|Default|SetFoundSpot (== (Utilities|Array|Length _outactors) 0))
      (Math|Integer|IncrementInt (Variables|Default|GetAttempts)))
    (if (Variables|Default|GetFoundSpot)
      (bind _returnvalue (Game|SpawnActorfromClass "/Game/Blueprints/Puzzles/DustSweeping/BP_Dust.BP_Dust_C" (Math|Conversions|ToTransform(Vector) (Variables|Default|GetCandidateLocation)) "Undefined" "MultiplyWithRoot" 0 0))
      (Utilities|Array|Add (Variables|Default|GetSpawnedDust) _returnvalue))))

(fn ConstructionScript)