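; Puzzle manager for dust sweeping that scatters dust and reports the puzzle solved once all of it is swept.
; On BeginPlay it tries to spawn a random number of BP_Dust actors in each DustZone-tagged actor's box, using collision-checked points that ignore dust already spawned.
; Each dust's sweep event removes it from the tracked array, and emptying that array calls PuzzleSolved on BP_GameMode.
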(event Custom|SweepedDust
  (params (DustRef :type BP%20Dust%20Object%20Reference))
  (CallFunction|RemoveDust DustRef))

(event EventBeginPlay
  (bind _outactors (Actor|GetAllActorswithTag "DustZone"))
  (for _array_element _outactors
    (for _index (range 0 (Math|Random|RandomIntegerinRange 3 12))
      (bind (_foundspot _location) (CallFunction|FindValidSpawnPoint (Actor|GetComponentbyClass _array_element "/Script/Engine.BoxComponent") "15.000000,15.000000,0.000000" (Utilities|Array|MakeArray "ObjectTypeQuery1" "ObjectTypeQuery2") (Variables|Default|GetSpawnedDust)))
      (if _foundspot
        (bind _returnvalue (Game|SpawnActorfromClass "/Game/Blueprints/Puzzles/DustSweeping/BP_Dust.BP_Dust_C" (Math|Conversions|ToTransform(Vector) _location) "Undefined" "MultiplyWithRoot" 0 0))
        (EventDispatchers|BindEventtoSweeped _returnvalue (delegate Custom|SweepedDust))
        (Utilities|Array|Add (Variables|Default|GetSpawnedDust) _returnvalue)))))

(fn ConstructionScript)

(fn RemoveDust
  (params (DustRef :type BP%20Dust%20Object%20Reference))
  (bind _spawneddust (Variables|Default|GetSpawnedDust))
  (Utilities|Array|RemoveItem _spawneddust DustRef)
  (if (<= (Utilities|Array|Length _spawneddust) 0)
    (bind _asbp_game_mode (Utilities|Casting|CastToBP_GameMode (Game|GetGameMode)))
    (Default|PuzzleSolved _asbp_game_mode)))