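; Bathroom sink locker furniture Blueprint with an interactable door and an item spawner component.
; Interacting with the door component toggles it through a FlipFlop that plays or reverses a Timeline, which lerps the door's relative yaw a quarter turn between closed and open.
; When the actor is destroyed, it tells the item spawner to clear its props.
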(event EventDestroyed
  (Default|ClearProps (Variables|Default|GetBPC_ItemSpawner)))

(event EventInteract
  (params (HitComponent :type Primitive%20Component%20Object%20Reference) (Location :type Vector :default "0, 0, 0") (HeldItem :type Actor%20Object%20Reference))
  (if (== HitComponent (Variables|Default|GetBathroom_SinkLocker_Doors))
    (Utilities|FlowControl|FlipFlop
      (:A
        (bind _open (Timeline|Timeline Play)
          (:Update
            (Transformation|SetRelativeRotation (Variables|Default|GetBathroom_SinkLocker_Doors) (Math|Rotator|MakeRotator 0.0 0.0 (Math|Float|Lerp 0.0 -9e+01 _open)) false false))))
      (:B
        (Timeline|Timeline Reverse)))))

(fn ConstructionScript)