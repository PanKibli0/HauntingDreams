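; BP_LockerTV is an interactable TV locker furniture piece with two swinging doors.
; Interact checks which door was hit, and a per-door FlipFlop plays or reverses its timeline with an open or close sound.
; Each timeline lerps door yaw to swing the left and right doors in opposite directions.
; On destruction, it clears props through its BPCItemSpawner component.
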(event EventDestroyed
  (Default|ClearProps (Variables|Default|GetBPC_ItemSpawner)))

(event EventInteract
  (params (HitComponent :type Primitive%20Component%20Object%20Reference) (Location :type Vector :default "0, 0, 0") (HeldItem :type Actor%20Object%20Reference))
  (if (== HitComponent (Variables|Default|GetLockerTV_DoorLeft))
    (Utilities|FlowControl|FlipFlop
      (:A
        (Audio|PlaySound2D "/Game/Audio/Sounds/Items/cabinet_open.cabinet_open" 1.0 1.0 0.0 0 0)
        (bind _open (Timeline|Timeline Play)
          (:Update
            (Transformation|SetRelativeRotation (Variables|Default|GetLockerTV_DoorLeft) (Math|Rotator|MakeRotator 0.0 0.0 (Math|Float|Lerp 0.0 9e+01 _open)) false false))))
      (:B
        (Audio|PlaySound2D "/Game/Audio/Sounds/Items/cabinet_close.cabinet_close" 1.0 1.0 0.0 0 0)
        (Timeline|Timeline Reverse)))
    (elif (== HitComponent (Variables|Default|GetLockerTV_DoorRight))
      (Utilities|FlowControl|FlipFlop
        (:A
          (Audio|PlaySound2D "/Game/Audio/Sounds/Items/cabinet_open.cabinet_open" 1.0 1.0 0.0 0 0)
          (bind _open_2 (Timeline|Timeline_0 Play)
            (:Update
              (Transformation|SetRelativeRotation (Variables|Default|GetLockerTV_DoorRight) (Math|Rotator|MakeRotator 0.0 0.0 (Math|Float|Lerp 0.0 -9e+01 _open_2)) false false))))
        (:B
          (Audio|PlaySound2D "/Game/Audio/Sounds/Items/cabinet_close.cabinet_close" 1.0 1.0 0.0 0 0)
          (Timeline|Timeline_0 Reverse))))))

(fn ConstructionScript)