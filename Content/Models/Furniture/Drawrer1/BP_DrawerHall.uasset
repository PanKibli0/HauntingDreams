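; Interactive hall drawer furniture with three shelves that the player opens and closes individually.
; The Interact event matches the hit component to a shelf, and that shelf's FlipFlop alternates open and close, each with a 2D sound.
; Each shelf has its own timeline, played or reversed to lerp its relative location along X.
; When the actor is destroyed, its item spawner component clears its props.
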(event EventDestroyed
  (Default|ClearProps (Variables|Default|GetBPC_ItemSpawner)))

(event EventInteract
  (params (HitComponent :type Primitive%20Component%20Object%20Reference) (Location :type Vector :default "0, 0, 0") (HeldItem :type Actor%20Object%20Reference))
  (if (== HitComponent (Variables|Default|GetDrawerShelf))
    (Utilities|FlowControl|FlipFlop
      (:A
        (Audio|PlaySound2D "/Game/Audio/Sounds/Items/drawer_open.drawer_open" 0.2 1.0 0.0 0 0)
        (bind _open (Timeline|TL_Open Play)
          (:Update
            (Transformation|SetRelativeLocation (Variables|Default|GetDrawerShelf) (Math|Vector|Lerp(Vector) "0, 0, 0" "40.000000,0.000000,0.000000" _open) false false))))
      (:B
        (Audio|PlaySound2D "/Game/Audio/Sounds/Items/drawer_close.drawer_close" 0.2 1.0 0.0 0 0)
        (Timeline|TL_Open Reverse)))
    (elif (== HitComponent (Variables|Default|GetDrawerShelf1))
      (Utilities|FlowControl|FlipFlop
        (:A
          (Audio|PlaySound2D "/Game/Audio/Sounds/Items/drawer_open.drawer_open" 0.2 1.0 0.0 0 0)
          (bind _open_2 (Timeline|TL_Open1 Play)
            (:Update
              (Transformation|SetRelativeLocation (Variables|Default|GetDrawerShelf1) (Math|Vector|Lerp(Vector) "0.000000,0.000000,34.000000" "40.000000,0.000000,34.000000" _open_2) false false))))
        (:B
          (Audio|PlaySound2D "/Game/Audio/Sounds/Items/drawer_close.drawer_close" 0.2 1.0 0.0 0 0)
          (Timeline|TL_Open1 Reverse)))
      (elif (== HitComponent (Variables|Default|GetDrawerShelf2))
        (Utilities|FlowControl|FlipFlop
          (:A
            (Audio|PlaySound2D "/Game/Audio/Sounds/Items/drawer_open.drawer_open" 0.2 1.0 0.0 0 0)
            (bind _open_3 (Timeline|TL_Open2 Play)
              (:Update
                (Transformation|SetRelativeLocation (Variables|Default|GetDrawerShelf2) (Math|Vector|Lerp(Vector) "0.000000,0.000000,68.000000" "40.000000,0.000000,68.000000" _open_3) false false))))
          (:B
            (Audio|PlaySound2D "/Game/Audio/Sounds/Items/drawer_close.drawer_close" 0.2 1.0 0.0 0 0)
            (Timeline|TL_Open2 Reverse)))))))

(fn ConstructionScript)