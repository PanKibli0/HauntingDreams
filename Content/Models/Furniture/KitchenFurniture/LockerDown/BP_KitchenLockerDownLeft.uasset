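; Interactive lower-left kitchen locker furniture Blueprint with a slim hinged door and a sliding shelf.
; The Interact event checks which component was hit, the left door or the shelf, and a FlipFlop for each alternates between playing and reversing its timeline.
; One timeline lerps the door's yaw to swing it open, the other lerps the shelf's relative location to slide it along X.
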(event EventInteract
  (params (HitComponent :type Primitive%20Component%20Object%20Reference))
  (if (== HitComponent (Variables|Default|GetLockerKitchen_DownSlim_DoorLeft))
    (Utilities|FlowControl|FlipFlop
      (:A
        (bind _open (Timeline|Timeline_0 Play)
          (:Update
            (Transformation|SetRelativeRotation (Variables|Default|GetLockerKitchen_DownSlim_DoorLeft) (Math|Rotator|MakeRotator 0.0 0.0 (Math|Float|Lerp 0.0 9e+01 _open)) false false))))
      (:B
        (Timeline|Timeline_0 Reverse)))
    (elif (== HitComponent (Variables|Default|GetLockerKitchen_Down_Shelf))
      (Utilities|FlowControl|FlipFlop
        (:A
          (bind _open_2 (Timeline|Timeline_1 Play)
            (:Update
              (Transformation|SetRelativeLocation (Variables|Default|GetLockerKitchen_Down_Shelf) (Math|Vector|Lerp(Vector) "0, 0, 0" "-40.000000,0.000000,0.000000" _open_2) false false))))
        (:B
          (Timeline|Timeline_1 Reverse))))))

(fn ConstructionScript)