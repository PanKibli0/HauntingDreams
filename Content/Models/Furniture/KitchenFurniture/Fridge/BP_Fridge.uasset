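; BP_Fridge is an interactable kitchen fridge with two doors that open and close separately.
; On BeginPlay it plays the fridge sound cue at its location.
; Interact checks which door component was hit, then a per-door FlipFlop alternates opening and closing.
; Each door has its own timeline that lerps its yaw to swing it open, reverses to close it, and plays matching open or close sounds.
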(event EventBeginPlay
  (Audio|PlaySoundatLocation "/Game/Audio/Sounds/Ambience/SC_Fridge.SC_Fridge" (Transformation|GetActorLocation) "0, 0, 0" 1.0 1.0 0.0 0 0 0 0))

(event EventInteract
  (params (HitComponent :type Primitive%20Component%20Object%20Reference) (Location :type Vector :default "0, 0, 0") (HeldItem :type Actor%20Object%20Reference))
  (if (== HitComponent (Variables|Default|GetFridgeDoorDown))
    (Utilities|FlowControl|FlipFlop
      (:A
        (Audio|PlaySound2D "/Game/Audio/Sounds/Items/fridge_open.fridge_open" 0.5 1.0 0.0 0 0)
        (bind _open (Timeline|Timeline Play)
          (:Update
            (Transformation|SetRelativeRotation (Variables|Default|GetFridgeDoorDown) (Math|Rotator|MakeRotator 0.0 0.0 (Math|Float|Lerp 0.0 -8e+01 _open)) false false))))
      (:B
        (Audio|PlaySound2D "/Game/Audio/Sounds/Items/fridge_close.fridge_close" 0.5 1.0 0.4 0 0)
        (Timeline|Timeline Reverse)))
    (elif (== HitComponent (Variables|Default|GetFridgeDoorUp))
      (Utilities|FlowControl|FlipFlop
        (:A
          (Audio|PlaySound2D "/Game/Audio/Sounds/Items/fridge_open.fridge_open" 0.5 1.0 0.0 0 0)
          (bind _open_2 (Timeline|Timeline_0 Play)
            (:Update
              (Transformation|SetRelativeRotation (Variables|Default|GetFridgeDoorUp) (Math|Rotator|MakeRotator 0.0 0.0 (Math|Float|Lerp 0.0 -8e+01 _open_2)) false false))))
        (:B
          (Audio|PlaySound2D "/Game/Audio/Sounds/Items/fridge_close.fridge_close" 0.5 1.0 0.3 0 0)
          (Timeline|Timeline_0 Reverse))))))

(fn ConstructionScript)