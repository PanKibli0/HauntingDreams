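; BP_WardrobeHall is a hall wardrobe furniture Blueprint with two doors that open and close independently on interaction.
; The Interact event compares the hit component to each door mesh to choose which one to move.
; Each door has its own FlipFlop that alternates between playing and reversing a Timeline, which lerps the door's relative yaw to swing it a quarter turn in opposite directions.
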(event EventInteract
  (params (HitComponent :type Primitive%20Component%20Object%20Reference) (Location :type Vector :default "0, 0, 0") (HeldItem :type Actor%20Object%20Reference))
  (if (== HitComponent (Variables|Default|GetWardrobe_DoorLeft))
    (Utilities|FlowControl|FlipFlop
      (:A
        (bind _open (Timeline|Timeline Play)
          (:Update
            (Transformation|SetRelativeRotation (Variables|Default|GetWardrobe_DoorLeft) (Math|Rotator|MakeRotator 0.0 0.0 (Math|Float|Lerp 0.0 9e+01 _open)) false false))))
      (:B
        (Timeline|Timeline Reverse)))
    (elif (== HitComponent (Variables|Default|GetWardrobe_DoorRight))
      (Utilities|FlowControl|FlipFlop
        (:A
          (bind _open_2 (Timeline|Timeline_0 Play)
            (:Update
              (Transformation|SetRelativeRotation (Variables|Default|GetWardrobe_DoorRight) (Math|Rotator|MakeRotator 0.0 0.0 (Math|Float|Lerp 0.0 -9e+01 _open_2)) false false))))
        (:B
          (Timeline|Timeline_0 Reverse))))))

(fn ConstructionScript)