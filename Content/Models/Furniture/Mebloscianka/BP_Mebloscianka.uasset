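; Interactable wall unit furniture (meblościanka) with doors and shelves that open and close.
; Interact passes a cooldown check, then component tags select a timeline that swings Right, Left or Middle parts or slides the two shelf types.
; Current transform decides open or close, and timelines move the last stored Target component.
; Destruction clears props through BPCItemSpawner; an older F3Shelf slide branch is left unconnected.
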(event EventDestroyed
  (Default|ClearProps (Variables|Default|GetBPC_ItemSpawner)))

(event EventInteract
  (params (HitComponent :type Primitive%20Component%20Object%20Reference))
  (bind _success (Default|CanInteract (Variables|Default|GetBPC_InteractionCooldown)))
  (if _success
    (Utilities|IsValid HitComponent
      (:Is%20Valid
        (bind _output_get (Variables|Default|SetTarget HitComponent))
        (if (Components|ComponentHasTag _output_get "Right")
          (if (!= (.Yaw (Math|Rotator|BreakRotator (Variables|/Script/Engine.SceneComponent|GetRelativeRotation _output_get))) 0.0)
            (bind _open (Timeline|Timeline ReverseFromEnd)
              (:Update
                (Transformation|SetRelativeRotation (Variables|Default|GetTarget) (Math|Rotator|Lerp(Rotator) "0, 0, 0" "0.000000,-83.000000,0.000000" _open) false false)))
            (else
              (Timeline|Timeline PlayFromStart)))
          (elif (Components|ComponentHasTag _output_get "Left")
            (if (!= (.Yaw (Math|Rotator|BreakRotator (Variables|/Script/Engine.SceneComponent|GetRelativeRotation _output_get))) 0.0)
              (bind _open_2 (Timeline|Timeline_0 ReverseFromEnd)
                (:Update
                  (Transformation|SetRelativeRotation (Variables|Default|GetTarget) (Math|Rotator|Lerp(Rotator) "0, 0, 0" "0.000000,83.000000,0.000000" _open_2) false false)))
              (else
                (Timeline|Timeline_0 PlayFromStart)))
            (elif (Components|ComponentHasTag _output_get "Middle")
              (if (!= (.Pitch (Math|Rotator|BreakRotator (Variables|/Script/Engine.SceneComponent|GetRelativeRotation _output_get))) 0.0)
                (bind _open_3 (Timeline|Timeline_1 ReverseFromEnd)
                  (:Update
                    (Transformation|SetRelativeRotation (Variables|Default|GetTarget) (Math|Rotator|MakeRotator 0.0 (Math|Float|Lerp 0.0 -9e+01 _open_3) 0.0) false false)))
                (else
                  (Timeline|Timeline_1 PlayFromStart)))
              (elif (Components|ComponentHasTag _output_get "Shelf")
                (if (!= (.X (Math|Vector|BreakVector (Variables|/Script/Engine.SceneComponent|GetRelativeLocation _output_get))) 7.0)
                  (bind _open_4 (Timeline|Timeline_3 Reverse)
                    (:Update
                      (Transformation|SetRelativeLocation (Variables|Default|GetTarget) (Math|Vector|Lerp(Vector) "7.000000,0.000000,0.000000" "40.000000,0.000000,0.000000" _open_4) false false)))
                  (else
                    (Timeline|Timeline_3 Play)))
                (elif (Components|ComponentHasTag _output_get "Shelf2")
                  (if (!= (.X (Math|Vector|BreakVector (Variables|/Script/Engine.SceneComponent|GetRelativeLocation _output_get))) 7.0)
                    (bind _open_5 (Timeline|Timeline_4 Reverse)
                      (:Update
                        (Transformation|SetRelativeLocation (Variables|Default|GetTarget) (Math|Vector|Lerp(Vector) "7.000000,0.000000,24.000000" "40.000000,0.000000,24.000000" _open_5) false false)))
                    (else
                      (Timeline|Timeline_4 Play))))))))))))

(fn ConstructionScript)