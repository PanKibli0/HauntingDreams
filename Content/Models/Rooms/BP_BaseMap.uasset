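; BP_BaseMap is one room segment in a looping level, configured on BeginPlay from the game mode's LoopSequence entry: lights, wall material, task ID and door lock.
; A box trigger fires once for the player, closing the door, spawning the next loop at an arrow and destroying the loop two back.
; Completing the matching task unlocks the door with a sound.
; A looping timer randomizes flickering lights, and a U-key debug unlock exists.
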(event OnComponentBeginOverlap(Box)
  (params (OverlappedComponent :type Primitive%20Component%20Object%20Reference) (OtherActor :type Actor%20Object%20Reference) (OtherComp :type Primitive%20Component%20Object%20Reference) (OtherBodyIndex :type Integer) (bFromSweep :type Boolean) (SweepResult :type Hit%20Result%20Structure%20%28by%20ref%29))
  (bind _doorref (Variables|Default|GetDoorRef))
  (if (and (== OtherActor (Pawn|GetControlledPawn (Game|GetPlayerController 0))) (not (Variables|Default|GetbeenTriggered)))
    (bind _asbp_game_mode (Utilities|Casting|CastToBP_GameMode (Game|GetGameMode)))
    (Variables|Default|SetbeenTriggered true)
    (Utilities|IsValid _doorref
      (:Is%20Valid
        (Default|CloseDoor _doorref))
      (:Is%20Not%20Valid
        _))
    (Utilities|FlowControl|Delay 1.0)
    (Variables|/Game/Player/BP_GameMode.BP_GameMode_C|SetCurrentLoopRef _asbp_game_mode self)
    (Utilities|FlowControl|Sequence
      (:then_0
        (Utilities|IsValid (Variables|Default|GetPrev2Loop)
          (:Is%20Valid
            (Utilities|FlowControl|Delay 2.0)
            (Default|ClearProps (Actor|GetComponentbyClass (Variables|Default|GetPrev2Loop) "/Game/Blueprints/Enviroment/BPC_ItemSpawner.BPC_ItemSpawner_C"))
            (Actor|DestroyActor (Variables|Default|GetPrev2Loop)))))
      (:then_1
        (bind _asbp_game_mode_2 (Utilities|Casting|CastToBP_GameMode (Game|GetGameMode)))
        (bind _spawnedactor (Default|SpawnNextLoop _asbp_game_mode_2 (Transformation|GetWorldTransform (Variables|Default|GetArrow))))
        (bind _asbp_base_map (Utilities|Casting|CastToBP_BaseMap _spawnedactor))
        (Variables|BP_BaseMap_C|SetPrev2Loop _asbp_base_map (Variables|Default|GetPrevLoop))
        (bind _output_get (Variables|BP_BaseMap_C|SetPrevLoop _asbp_base_map self))
        (bind _asbp_door (Utilities|Casting|CastToBP_Door _output_get))
        (Variables|/Game/Blueprints/Enviroment/BP_Door.BP_Door_C|SetisLocked _asbp_door true)
        (Default|CloseDoor _asbp_door)))))

(event Custom|StartFlicker
  ;[0.15 0.1255 0 0.5] Light flickering
  (Utilities|Time|ClearandInvalidateTimerbyHandle (Variables|Default|GetFlickerHandle))
  (bind _returnvalue (Utilities|Time|SetTimerbyEvent (delegate Custom|FlickerTick) 0.5 true))
  (Variables|Default|SetFlickerHandle _returnvalue))

(event Custom|FlickerTick
  ;[0.15 0.1255 0 0.5] Light flickering
  (for _array_element (Variables|Default|GetFlickeringLights)
    (Rendering|Components|Light|SetIntensity _array_element (Math|Random|RandomFloatinRange 0.0 5e+03))
    (Rendering|SetVisibility _array_element (Math|Random|RandomBoolwithWeight 0.7) false)))

(event Custom|UnlockDoors
  (Variables|/Game/Blueprints/Enviroment/BP_Door.BP_Door_C|SetisLocked (Variables|Default|GetDoorRef) false))

(event Custom|NotifyTaskCompleted
  (params (TaskID :type Name))
  (bind _doorref (Variables|Default|GetDoorRef))
  (if (== TaskID (Variables|Default|GetCurrentTaskID))
    (Variables|/Game/Blueprints/Enviroment/BP_Door.BP_Door_C|SetisLocked _doorref false)
    (Audio|PlaySoundatLocation 0 (Transformation|GetWorldLocation (Variables|/Game/Blueprints/Enviroment/BP_Door.BP_Door_C|GetDefaultSceneRoot _doorref)) "0, 0, 0" 1.0 1.0 0.0 0 0 0 0)))

(event EventBeginPlay
  ;[0 0.15 0.01354 0.5] EVENT BEGINPLAY
  (bind _returnvalue (Actor|GetActorOfClass "/Game/Blueprints/Enviroment/BP_Door.BP_Door_C"))
  (Variables|Default|SetDoorRef _returnvalue)
  (CallFunction|ApplyLoopChanges))

(event Input|KeyboardEvents|U
  (params (Key :type Key%20Structure :default "None"))
  (:Pressed
    (CallFunction|UnlockDoors)
    (Development|PrintString "Hello")))

(fn ConstructionScript)

(fn ApplyLoopChanges
  (Utilities|Array|Clear (Variables|Default|GetFlickeringLights))
  (bind _asbp_game_mode (Utilities|Casting|CastToBP_GameMode (Game|GetGameMode)))
  (Utilities|FlowControl|Sequence
    (:then_0
      (for _array_element (Actor|GetComponentsByClass "/Script/Engine.LightComponent")
        (Utilities|IsValid _array_element
          (:Is%20Valid
            (Rendering|Components|Light|SetLightColor _array_element (Variables|/Game/DataAssets/PDA_LoopConfig.PDA_LoopConfig_C|GetLightColor (Utilities|Array|Get(acopy) (Variables|/Game/Player/BP_GameMode.BP_GameMode_C|GetLoopSequence _asbp_game_mode) (Variables|/Game/Player/BP_GameMode.BP_GameMode_C|GetCurrentLoopIndex _asbp_game_mode))) true)
            (switch Utilities|FlowControl|Switch|SwitchonE_LightEnum (Variables|/Game/DataAssets/PDA_LoopConfig.PDA_LoopConfig_C|GetLightState (Utilities|Array|Get(acopy) (Variables|/Game/Player/BP_GameMode.BP_GameMode_C|GetLoopSequence _asbp_game_mode) (Variables|/Game/Player/BP_GameMode.BP_GameMode_C|GetCurrentLoopIndex _asbp_game_mode)))
              (:NewEnumerator0
                (Rendering|Components|Light|SetIntensity _array_element 0.0))
              (:NewEnumerator1
                (Rendering|Components|Light|SetIntensity _array_element 5e+02))
              (:NewEnumerator2
                (Utilities|Array|AddUnique (Variables|Default|GetFlickeringLights) _array_element))))))
      (CallFunction|StartFlicker))
    (:then_1
      (Utilities|IsValid (Utilities|Array|Get(acopy) (Variables|/Game/Player/BP_GameMode.BP_GameMode_C|GetLoopSequence _asbp_game_mode) (Variables|/Game/Player/BP_GameMode.BP_GameMode_C|GetCurrentLoopIndex _asbp_game_mode))
        (:Is%20Valid
          (if (Variables|/Game/DataAssets/PDA_LoopConfig.PDA_LoopConfig_C|GetIsTaskRequired (Utilities|Array|Get(acopy) (Variables|/Game/Player/BP_GameMode.BP_GameMode_C|GetLoopSequence _asbp_game_mode) (Variables|/Game/Player/BP_GameMode.BP_GameMode_C|GetCurrentLoopIndex _asbp_game_mode)))
            (bind _asbp_door (Utilities|Casting|CastToBP_Door (Variables|/Script/Engine.ChildActorComponent|GetChildActor (Variables|Default|GetBP_Door))))
            (Utilities|IsValid _asbp_door
              (:Is%20Valid
                (Variables|Default|SetCurrentTaskID (Variables|/Game/DataAssets/PDA_LoopConfig.PDA_LoopConfig_C|GetTaskID (Utilities|Array|Get(acopy) (Variables|/Game/Player/BP_GameMode.BP_GameMode_C|GetLoopSequence _asbp_game_mode) (Variables|/Game/Player/BP_GameMode.BP_GameMode_C|GetCurrentLoopIndex _asbp_game_mode))))
                (Variables|/Game/Blueprints/Enviroment/BP_Door.BP_Door_C|SetisLocked _asbp_door (Variables|/Game/DataAssets/PDA_LoopConfig.PDA_LoopConfig_C|GetIsDoorLocked (Utilities|Array|Get(acopy) (Variables|/Game/Player/BP_GameMode.BP_GameMode_C|GetLoopSequence _asbp_game_mode) (Variables|/Game/Player/BP_GameMode.BP_GameMode_C|GetCurrentLoopIndex _asbp_game_mode))))
                (Development|PrintString "ZABLOKOWANO DRZWI"))))
          (Utilities|Array|AddUnique (Variables|Default|GetFlickeringLights) _array_element))))
    (:then_2
      (Utilities|IsValid (Variables|/Game/DataAssets/PDA_LoopConfig.PDA_LoopConfig_C|GetWallMaterial (Utilities|Array|Get(acopy) (Variables|/Game/Player/BP_GameMode.BP_GameMode_C|GetLoopSequence _asbp_game_mode) (Variables|/Game/Player/BP_GameMode.BP_GameMode_C|GetCurrentLoopIndex _asbp_game_mode)))
        (:Is%20Valid
          (bind _asbp_salon (Utilities|Casting|CastToBP_Salon (Variables|/Script/Engine.ChildActorComponent|GetChildActor (Variables|Default|GetBP_Salon))))
          (Default|UpdateWalls _asbp_salon (Variables|/Game/DataAssets/PDA_LoopConfig.PDA_LoopConfig_C|GetWallMaterial (Utilities|Array|Get(acopy) (Variables|/Game/Player/BP_GameMode.BP_GameMode_C|GetLoopSequence _asbp_game_mode) (Variables|/Game/Player/BP_GameMode.BP_GameMode_C|GetCurrentLoopIndex _asbp_game_mode)))))))))