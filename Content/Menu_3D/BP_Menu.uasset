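; 3D menu station actor that moves the player's view between linked menus and launches the game from its widget.
; Widget events either blend the camera to a menu in LinkedMenus or to the StartGame target before opening the "Basic" level.
; Actor collision is enabled only on the starting or arrived-at menu.
; An optional child-actor door swings open via a timeline on game start, or on transitions when OpenDoorOnMenu is set.
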(event Custom|Transition
  (params (NewParam :type BP%20Menu%20Object%20Reference))
  (Collision|SetActorEnableCollision false)
  (Utilities|FlowControl|Sequence
    (:then_0
      (Game|Player|SetViewTargetwithBlend (Game|GetPlayerController 0) NewParam 2.0 "VTBlend_EaseInOut" 2.0 false)
      (Utilities|FlowControl|Delay 2.0)
      (Collision|SetActorEnableCollision NewParam true))
    (:then_1
      (if (Variables|Default|GetOpenDoorOnMenu)
        (CallFunction|AnimateDoorOpen)))))

(event Custom|OnTransitionBetweenMenus
  (params (MenuIndex :type Integer))
  (if (Utilities|Array|IsValidIndex (Variables|Default|GetLinkedMenus) MenuIndex)
    (CallFunction|Transition (Utilities|Array|Get(acopy) (Variables|Default|GetLinkedMenus) MenuIndex))))

(event Custom|AnimateDoorOpen
  (bind _asbp_doors (Utilities|Casting|CastToBP_Doors (Variables|/Script/Engine.ChildActorComponent|GetChildActor (Variables|Default|GetBP_Doors))))
  (bind _newtrack_0 (Timeline|Timeline Play)
    (:Update
      (Transformation|SetRelativeRotation (Variables|/Game/Models/Doors/BP_Doors.BP_Doors_C|GetDoors _asbp_doors) (Math|Rotator|MakeRotator (.Roll (Math|Rotator|BreakRotator (Variables|/Script/Engine.SceneComponent|GetRelativeRotation (Variables|/Game/Models/Doors/BP_Doors.BP_Doors_C|GetDoors _asbp_doors)))) (.Pitch (Math|Rotator|BreakRotator (Variables|/Script/Engine.SceneComponent|GetRelativeRotation (Variables|/Game/Models/Doors/BP_Doors.BP_Doors_C|GetDoors _asbp_doors)))) (Math|Float|Lerp 0.0 -9e+01 _newtrack_0)) false false))))

(event Custom|StartGameSequence
  (bind _returnvalue (Game|GetPlayerController 0))
  (Variables|/Script/Engine.PlayerController|SetbShowMouseCursor _returnvalue false)
  (Input|SetInputModeGameOnly _returnvalue false)
  (Collision|SetActorEnableCollision false)
  (CallFunction|AnimateDoorOpen)
  (Game|Player|SetViewTargetwithBlend (Game|GetPlayerController 0) (Variables|Default|GetStartGame) 2.0 "VTBlend_Linear" 2.0 false)
  (Utilities|FlowControl|Delay 2.0)
  (Game|OpenLevel(byName) "Basic"))

(event EventBeginPlay
  (if (Variables|Default|GetIsStartingMenu)
    (Collision|SetActorEnableCollision true)
    (else
      (Collision|SetActorEnableCollision false)))
  (if (Variables|Default|GetHasDoors)
    _
    (else
      (Components|DestroyComponent (Variables|Default|GetBP_Doors))))
  (bind _asmenu_3d_base_widget (Utilities|Casting|CastToMenu3D_Base_Widget (UserInterface|GetUserWidgetObject (Variables|Default|GetWidget))))
  (EventDispatchers|BindEventtoTransitiontoLinkedMenu _asmenu_3d_base_widget (delegate Custom|OnTransitionBetweenMenus))
  (EventDispatchers|BindEventtoOnStartGameClicked _asmenu_3d_base_widget (delegate Custom|StartGameSequence)))

(fn ConstructionScript)