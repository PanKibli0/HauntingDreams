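; BP_SpiderCoin is an AI-controlled spider that reacts to being lit.
; It registers with BP_LightManager on BeginPlay and unregisters on EndPlay.
; Its seen-by-light and lost-light events write the IsLit flag and light hit location to the AI controller's Blackboard.
; An unconnected debug branch can force the lit state.
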(event Custom|OnSeenByLight
  (params (HitLocation :type Vector))
  (bind _asaicontroller (Utilities|Casting|CastToAIController (Pawn|GetController)))
  (AI|Components|Blackboard|SetValueasBool (AI|GetBlackboard _asaicontroller) (Variables|Default|GetIsLit) true)
  (AI|Components|Blackboard|SetValueasVector (AI|GetBlackboard _asaicontroller) (Variables|Default|GetLightHitLocation) HitLocation))

(event Custom|OnLostLight
  (bind _asaicontroller (Utilities|Casting|CastToAIController (Pawn|GetController)))
  (AI|Components|Blackboard|SetValueasBool (AI|GetBlackboard _asaicontroller) (Variables|Default|GetIsLit) false))

(event EventEndPlay
  (params (EndPlayReason :type EEndPlayReason%20Enum :default "Destroyed"))
  (bind _returnvalue (Actor|GetActorOfClass "/Game/Blueprints/BP_LightManager.BP_LightManager_C"))
  (Default|UnregisterSpider _returnvalue self))

(event EventTick
  (params (DeltaSeconds :type Float%20%28single-precision%29)))

(event EventBeginPlay
  (bind _returnvalue (Actor|GetActorOfClass "/Game/Blueprints/BP_LightManager.BP_LightManager_C"))
  (Default|RegisterSpider _returnvalue self))

(fn ConstructionScript)